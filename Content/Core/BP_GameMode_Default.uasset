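; Default game mode that handles saving and loading of the player character's state.
; SaveGame loads or creates an SG_PlayerSave for the player slot and has it capture the character's state.
; LoadGame restores from that cached object without reading the slot, then sends an aggro reset to every NPC's AI controller, marked WIP.
; Per-level saving by level name exists only as unconnected nodes.
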(event `Event Save Game`
  (bind _returnvalue (`GameplayStatics.GetPlayerCharacter` 0))
  ;[0.05127 0.05127 0.05127] Saving
  (bind _returnvalue_2 (`GameplayStatics.DoesSaveGameExist` (`self.PlayerSaveName`)))
  (if _returnvalue_2
    (bind _returnvalue_3 (`GameplayStatics.LoadGameFromSlot` (`self.PlayerSaveName`)))
    (bind _assg_player_state_save (cast `/Game/Core/Saves/SG_PlayerSave` _returnvalue_3))
    (bind _output_get (set `self.PlayerSave` _assg_player_state_save))
    (`/Game/Core/Saves/SG_PlayerSave.SavePlayerCharacterState` _output_get _returnvalue)
    (else
      (bind _returnvalue_4 (`GameplayStatics.CreateSaveGameObject` "/Game/Core/Saves/SG_PlayerSave.SG_PlayerSave_C"))
      (bind _output_get_2 (set `self.PlayerSave` _returnvalue_4))
      (`/Game/Core/Saves/SG_PlayerSave.SavePlayerCharacterState` _output_get_2 _returnvalue))))

(event `Event Load Game`
  ;[0.05127 0.05127 0.05127] Saving
  (`/Game/Core/Saves/SG_PlayerSave.LoadPlayerCharacterState` (`self.PlayerSave`) (`GameplayStatics.GetPlayerCharacter` 0))
  ;[1 0 0] WIP
  (bind _outactors (`GameplayStatics.GetAllActorsOfClass` "/Game/AI/BP_NPC_Parent.BP_NPC_Parent_C"))
  (for _array_element _outactors
    (message `/Game/AI/BPI_AI.AggroReset` (`AIBlueprintHelperLibrary.GetAIController` _array_element))))

(fn `UserConstructionScript`)