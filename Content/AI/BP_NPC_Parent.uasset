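; Parent NPC character Blueprint that configures faction, gendered mesh and weapon, and handles movement speeds, timed attacks, takedowns and ragdolling.
; BPCHealth knockback and launches trigger physics ragdoll, which polls until slow and conscious, then recovers via pose snapshot and trace-selected get-up montage.
; Consciousness changes update the awareness widget, AIC_NPC blackboard and anim class.
; Losing consciousness stops AI and drops equipment by spawning a duplicate (work in progress).
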(event `self.ReceiveBeginPlay`
  (`self.Link Widget Awareness to Character`)
  (add `/Game/Universal/BPC_Health.EventKnockback` (`self.BPC_Health`) (delegate `Event Knockback`)))

(event `Event Knockback`
  (`self.Event Ragdoll`))

(event `/Game/AI/BPI_AI.LookAt`
  (params (`LookAt?` :type Boolean) (LookAtActor :type "Actor Object Reference"))
  ;[1 1 1] Sets actor to look at
  (if `LookAt?`
    (set `self.LookAtActor` LookAtActor)
    (else
      ;[1 1 1] If no (currently enemy) actors nearby
      ; Should probably take the nearest character instead. Failing that, leave blank
      (set `self.LookAtActor` null))))

(event `self.ReceiveTick`
  (params (DeltaSeconds :type "Float (single-precision)")))

(event `/Game/AI/BPI_AI.SetMovementCategory`
  (params (MovementCategory :type "/Game/AI/Behaviour/Pathfinding/Enum_MovementCategory Enum" :default "NewEnumerator0"))
  ;[1 1 1] Runs whenever movement category is changed, e.g. walking to combat
  (set `self.MovementType` MovementCategory)
  (set `CharacterMovementComponent.MaxWalkSpeed` (select `/Game/AI/Behaviour/Pathfinding/Enum_MovementCategory` (`self.MovementType`) :`NewEnumerator0` (`self.WalkSpeed`) :`NewEnumerator1` (`self.SearchSpeed`) :`NewEnumerator2` (`self.CombatSpeed`)) (`self.CharacterMovement`)))

(event `/Game/Universal/Interact/BPI_Interact.LootNPC`
  ;[1 1 1] Player Interact with NPC
)

(event `self.OnLaunched`
  (params (LaunchVelocity :type "Vector Structure") (bXYOverride :type Boolean) (bZOverride :type Boolean))
  (bind _mesh (`self.Mesh`))
  (bind _returnvalue (select `bool` (> (`KismetMathLibrary.Dot_VectorVector` LaunchVelocity (`self.GetActorForwardVector`)) 0.0) :!type "AnimMontage Object Reference"))
  ;[1 1 1] Ragdoll
  (if (`SceneComponent.IsSimulatingPhysics` (`self.Mesh`) "None")
    (`PrimitiveComponent.AddImpulseAtLocation` _mesh (* LaunchVelocity 25.0) (`SceneComponent.GetSocketLocation` _mesh "spine_02") "spine_02")
    (else
      (`self.PlayAnimMontage` _returnvalue)))
  (`KismetSystemLibrary.Delay` (select `bool` (`KismetSystemLibrary.IsValid` _returnvalue) :`false` 0.5 :`true` (`AnimSequenceBase.SequenceLength` _returnvalue)))
  (`self.Event Ragdoll`))

(event `/Game/AI/BPI_AI.Attack`
  (bind _childactor (`ChildActorComponent.ChildActor` (`self.Item`)))
  ;[1 1 1] Combat
  (if (not (`self.Attacking?`))
    (set `self.Attacking?` true)
    (message `/Game/Items/BPI_Item.Trigger` _childactor true)
    (`KismetSystemLibrary.Delay` 1.0)
    (message `/Game/Items/BPI_Item.Trigger` _childactor false)
    (`KismetSystemLibrary.Delay` 1.0)
    (set `self.Attacking?` false)))

(event `/Game/Universal/Interact/BPI_Interact.TalkNPC`
  ;[1 1 1] Player Interact with NPC
)

(event `Event Ragdoll`
  ;[1 1 1] Ragdoll
  (`PrimitiveComponent.SetCollisionEnabled` (`self.CapsuleComponent`) "NoCollision")
  (set `self.Ragdolling?` true)
  (`PrimitiveComponent.SetSimulatePhysics` (`self.Mesh`) true)
  (`CharacterMovementComponent.DisableMovement` (`self.CharacterMovement`))
  (`self.Event While Ragdolling`))

(event `/Game/Universal/Interact/BPI_Interact.TakedownNPC`
  (params (`Lethal?` :type Boolean))
  (bind _bpc_health (`self.BPC_Health`))
  ;[1 1 1] Player Interact with NPC
  ;;[1 1 1] Player takedown NPC (to be complexified)
  (if `Lethal?`
    (`/Game/Universal/BPC_Health.Event Death` _bpc_health)
    (else
      (`/Game/Universal/BPC_Health.Event Unconscious` _bpc_health))))

(event `Event Ragdoll Recover`
  (bind _mesh (`self.Mesh`))
  (bind _returnvalue (`SceneComponent.GetSocketLocation` _mesh "pelvis"))
  ;[1 1 1] Ragdoll
  (`PrimitiveComponent.SetSimulatePhysics` (`self.Mesh`) false)
  (bind (_outhit _returnvalue_2) (`KismetSystemLibrary.LineTraceSingle` _returnvalue (+ _returnvalue (* (`KismetMathLibrary.GetRightVector` (`SceneComponent.GetSocketRotation` _mesh "pelvis")) 50.0)) "TraceTypeQuery1"))
  (set `self.RagdollTickFlag` false)
  (`self.UpdateCapsuleLocation`)
  (`SceneComponent.K2_AttachToComponent` (`self.Mesh`) (`self.CapsuleComponent`) "None" "KeepRelative" "KeepRelative" "KeepRelative" true)
  (`SceneComponent.K2_SetRelativeLocationAndRotation` (`self.Mesh`) (0.0 0.0 -89.0) (struct :`Yaw` 270.0) false false)
  (`AnimInstance.SavePoseSnapshot` (`SkeletalMeshComponent.GetAnimInstance` (`self.Mesh`)) "RagdollFinalPose")
  (if _returnvalue_2
    (bind _returnvalue_3 (`self.PlayAnimMontage` "/Game/Animations/Mixamo/GettingUpFront_UE_Montage.GettingUpFront_UE_Montage"))
    (`KismetSystemLibrary.Delay` _returnvalue_3)
    (else
      (bind _returnvalue_4 (`self.PlayAnimMontage` "/Game/Animations/Mixamo/GettingUpBack_UE_Montage.GettingUpBack_UE_Montage"))
      (`KismetSystemLibrary.Delay` _returnvalue_4)))
  (if (`SceneComponent.IsSimulatingPhysics` (`self.Mesh`) "None")
    (`self.Event While Ragdolling`)
    (else
      (set `self.Ragdolling?` false)
      (`PrimitiveComponent.SetCollisionEnabled` (`self.CapsuleComponent`) "QueryAndPhysics")
      (`CharacterMovementComponent.SetMovementMode` (`self.CharacterMovement`) "MOVE_Walking" 0))))

(event `Event While Ragdolling`
  (bind _conscious_ (`/Game/Universal/BPC_Health.Conscious?` (`self.BPC_Health`)))
  ;[1 1 1] Ragdoll
  (if (not (`self.RagdollTickFlag`))
    (set `self.RagdollTickFlag` true)
    (`self.UpdateCapsuleLocation`)
    (`KismetSystemLibrary.Delay` 2.0)
    (if (and _conscious_ (<= (`self.MeshVelocity`) 20.0))
      (`self.Event Ragdoll Recover`)
      (elif _conscious_
        (set `self.RagdollTickFlag` false)
        (`self.Event While Ragdolling`)))))

(event `/Game/AI/BPI_AI.SetConscious`
  (params (`Conscious?` :type Boolean))
  (bind _item (`self.Item`))
  (bind _childactor (`ChildActorComponent.ChildActor` _item))
  (`self.SetConsciousness` `Conscious?`)
  (if `Conscious?`
    (goto _label :!via `Reset`)))

(event `Event Drop Equipment`
  (bind _item (`self.Item`))
  (bind _childactor (`ChildActorComponent.ChildActor` _item))
  ;[1 1 1] Work in progress - destroys equipment and spawns in a duplicate
  (`/Engine/EditorBlueprintResources/StandardMacros.DoOnce` false :!label _label
    (:`Completed`
      (`|SpawnActorFromClass` (`ChildActorComponent.ChildActorClass` _item) (`self.GetTransform` _childactor) "AlwaysSpawn" "MultiplyWithRoot" null null)
      (`self.K2_DestroyActor` _childactor))))

(fn `Fall Damage`)

(fn `Link Widget Awareness to Character`
  (bind _aswbp_awareness (cast `/Game/AI/Widgets/WBP_Awareness` (`WidgetComponent.GetUserWidgetObject` (`self.WidgetAwareness`))))
  (bind _asaic_npc (cast `/Game/AI/Behaviour/AIC_NPC` (`AIBlueprintHelperLibrary.GetAIController` self)))
  (set `/Game/AI/Widgets/WBP_Awareness.As AIC NPC` _asaic_npc _aswbp_awareness))

(fn `RandomiseGender`
  (params (`IncludeRobot?` :type Boolean))
  (set `self.Gender` (select `bool` (and (`KismetMathLibrary.RandomBoolWithWeight` 0.25) `IncludeRobot?`) :`false` (select `int` (`KismetMathLibrary.RandomInteger` 2) :`0` "NewEnumerator1" :`1` "NewEnumerator0" :!type "/Game/Universal/Enum_Gender Enum") :`true` (select `int` (`KismetMathLibrary.RandomInteger` 3) :`0` "NewEnumerator1" :`1` "NewEnumerator0" :`2` "NewEnumerator3" :!type "/Game/Universal/Enum_Gender Enum"))))

(fn `SetConsciousness`
  (params (`Conscious?` :type Boolean))
  (bind _returnvalue (`self.GetComponentByClass` (`self.GetOwner`) "/Script/Engine.SkeletalMeshComponent"))
  (bind _returnvalue_2 (`AIBlueprintHelperLibrary.GetAIController` self))
  (`SceneComponent.SetVisibility` (`self.WidgetAwareness`) `Conscious?` true)
  (`self.Event Ragdoll`)
  (`BlackboardComponent.SetValueAsBool` (`AIController.Blackboard` _returnvalue_2) "Conscious?" (`local.Conscious?`))
  (`/Engine/EditorBlueprintResources/StandardMacros.IsValid` _returnvalue
    (:`Is Valid`
      (`SkeletalMeshComponent.SetAnimInstanceClass` _returnvalue (select `bool` (`local.Conscious?`) :`true` "/Game/Animations/ABP_MotionMatching.ABP_MotionMatching_C" :!type "Object Class Reference")))
    (:`Is Not Valid`
      _))
  ;[1 1 1] Runs if owner is unconscious
  (if (not (`local.Conscious?`))
    (`Controller.StopMovement` _returnvalue_2)
    (`BrainComponent.StopLogic` (`AIController.BrainComponent` _returnvalue_2) "Died")
    ;[1 1 1] Stop attacking
    (message `/Game/Items/BPI_Item.Trigger` (`ChildActorComponent.ChildActor` (`self.Item`)) false)
    (`self.Event Drop Equipment`)))

(fn `UpdateCapsuleLocation`
  (bind _capsulecomponent (`self.CapsuleComponent`))
  (bind _returnvalue (`SceneComponent.GetSocketLocation` (`self.Mesh`) "root"))
  (bind (_outhit _returnvalue_2) (`KismetSystemLibrary.LineTraceSingle` _returnvalue (+ _returnvalue (0.0 0.0 -100.0)) "TraceTypeQuery1"))
  (if _returnvalue_2
    (set `self.GroundLocation` (`.Location` (`GameplayStatics.BreakHitResult` _outhit)))
    (else
      (set `self.GroundLocation` _returnvalue)))
  (`SceneComponent.K2_SetWorldLocation` _capsulecomponent (+ (* (`KismetMathLibrary.Vector_Up`) (`CapsuleComponent.CapsuleHalfHeight` _capsulecomponent)) (`self.GroundLocation`)) true false))

(fn `UserConstructionScript`
  (locals (`RandomiseGender?` :type Boolean :default true))
  (bind _bpc_inventory (`self.BPC_Inventory`))
  (bind (_currentitem_name _currentitem_icon _currentitem_description _currentitem_itemclass _currentitem_animation) (break `/Game/Items/Struct_Item` (`/Game/Items/BPC_Inventory.CurrentItem` _bpc_inventory)))
  (`|ExecutionSequence`
    (:`then_0`
      (set `/Game/Universal/Factions/BPC_Faction.Faction` (`self.Faction`) (`self.BPC_Faction`))
      (`ActorComponent.K2_DestroyComponent` (`self.3rdPersonCamera`)))
    (:`then_1`
      (set `/Game/Items/BPC_Inventory.FiniteAmmo?` false (`self.BPC_Inventory`))
      (`/Game/Items/BPC_Inventory.SetCurrentItem` _bpc_inventory (`.RowName` (break `DataTableRowHandle` (`self.Weapon`))) (0.0 0.0))
      (`ChildActorComponent.SetChildActorClass` (`self.Item`) (`|ConvertAsset` _currentitem_itemclass))
      (set `self.ItemAnim` _currentitem_animation))
    (:`then_2`
      (if (`local.RandomiseGender?`)
        (`self.RandomiseGender` false))
      (`SkeletalMeshComponent.SetSkeletalMeshAsset` (`self.Mesh`) (select `/Game/Universal/Enum_Gender` (`self.Gender`) :`NewEnumerator0` "/Game/Characters/Mannequins/Meshes/SKM_Manny.SKM_Manny" :`NewEnumerator1` "/Game/Characters/Mannequins/Meshes/SKM_Quinn.SKM_Quinn" :!type "SkeletalMesh Object Reference")))))