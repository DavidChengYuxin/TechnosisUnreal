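; Level streaming trigger volume that swaps sublevels when BP_ThirdPersonCharacter overlaps the actor or its Box component.
; Both overlap events feed one chain that asynchronously loads LevelToLoad as visible, then unloads LevelCurrent without blocking.
; Between load and unload it disables input and pauses, then immediately re-enables input and unpauses, with no wait between.
; The cast is tied to that character class, marked for replacement if the character changes.
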(event `self.ReceiveActorBeginOverlap`
  (params (OtherActor :type "Actor Object Reference"))
  ;[1 1 1] Replace if BP for character changes
  (cast `/Game/ThirdPerson/Blueprints/BP_ThirdPersonCharacter` OtherActor)
  (`GameplayStatics.LoadStreamLevelBySoftObjectPtr` (`self.LevelToLoad`) true :!label _label)
  (`self.DisableInput` (`GameplayStatics.GetPlayerController` 0))
  (`GameplayStatics.SetGamePaused` true)
  (`self.EnableInput` (`GameplayStatics.GetPlayerController` 0))
  (`GameplayStatics.SetGamePaused` false)
  (`GameplayStatics.UnloadStreamLevelBySoftObjectPtr` (`self.LevelCurrent`)))

(event `self.Box.OnComponentBeginOverlap`
  (params (OverlappedComponent :type "PrimitiveComponent Object Reference") (OtherActor :type "Actor Object Reference") (OtherComp :type "PrimitiveComponent Object Reference") (OtherBodyIndex :type Integer) (bFromSweep :type Boolean) (SweepResult :type "HitResult Structure (by ref)"))
  ;[1 1 1] Replace if BP for character changes
  (cast `/Game/ThirdPerson/Blueprints/BP_ThirdPersonCharacter` OtherActor)
  (goto _label))

(fn `UserConstructionScript`)