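; BP_OilBarrel is an explosive barrel prop that leaves oil puddles when it hits things.
; On Hit, a short downward trace spawns BP_OilPuddle on the surface below unless one already overlaps, then decrements Uses, which this graph never checks.
; Kinetic, fire, electric or armor-piercing damage triggers a one-time explosion: radial armor-piercing and fire damage, AI noise, effect, sound, then destruction.
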(event `self.ReceiveHit`
  (params (MyComp :type "PrimitiveComponent Object Reference") (Other :type "Actor Object Reference") (OtherComp :type "PrimitiveComponent Object Reference") (bSelfMoved :type Boolean) (HitLocation :type "Vector Structure") (HitNormal :type "Vector Structure") (NormalImpulse :type "Vector Structure") (Hit :type "HitResult Structure (by ref)"))
  (bind _returnvalue (`SceneComponent.K2_GetComponentLocation` (`self.Mesh`)))
  (`parent.ReceiveHit` MyComp Other OtherComp bSelfMoved HitLocation HitNormal NormalImpulse Hit)
  (bind (_outhit _returnvalue_2) (`KismetSystemLibrary.LineTraceSingle` _returnvalue (+ _returnvalue (* (`KismetMathLibrary.Vector_Down`) 50.0)) "TraceTypeQuery1" false (`|MakeArray` self :!type "Actor Object Reference")))
  (if _returnvalue_2
    (if (== (`KismetArrayLibrary.Array_Length` (`self.GetOverlappingActors` "/Game/ElementalDamage/Fire/BP_OilPuddle.BP_OilPuddle_C")) 0)
      (`|SpawnActorFromClass` "/Game/ElementalDamage/Fire/BP_OilPuddle.BP_OilPuddle_C" (`KismetMathLibrary.MakeTransform` (`.Location` (`GameplayStatics.BreakHitResult` _outhit))) "Undefined" "MultiplyWithRoot" null null)
      (`/Engine/EditorBlueprintResources/StandardMacros.DecrementInt` (`self.Uses`)))))

(event `self.ReceiveAnyDamage`
  (params (Damage :type "Float (single-precision)") (DamageType :type "DamageType Object Reference") (InstigatedBy :type "Controller Object Reference") (DamageCauser :type "Actor Object Reference"))
  (`/Game/Universal/BPML_Universal.SwitchOnElementalDamage` DamageType
    (:`Kinetic`
      _)
    (:`Fire`
      _)
    (:`Electricity`
      _)
    (:`ArmorPiercing`
      _))
  (`self.Event Explode` InstigatedBy DamageCauser))

(event `Event Explode`
  (params (InstigatedBy :type "Controller Object Reference") (DamageCauser :type "Actor Object Reference"))
  (bind _damage_inner_radius (`self.Damage Inner Radius`))
  (bind _damage_outer_radius (`self.Damage Outer Radius`))
  (bind _damage_falloff (`self.Damage Falloff`))
  (bind _returnvalue (`SceneComponent.K2_GetComponentLocation` (`self.Mesh`)))
  (bind _array (`|MakeArray` self :!type "Actor Object Reference"))
  (`/Engine/EditorBlueprintResources/StandardMacros.DoOnce` false
    (:`Completed`
      (`GameplayStatics.ApplyRadialDamageWithFalloff` 60.0 0.0 _returnvalue _damage_inner_radius _damage_outer_radius _damage_falloff "/Game/ElementalDamage/ArmorPiercing/DTBP_ArmorPiercing.DTBP_ArmorPiercing_C" _array DamageCauser InstigatedBy)
      (`GameplayStatics.ApplyRadialDamageWithFalloff` 15.0 0.5 _returnvalue _damage_inner_radius _damage_outer_radius _damage_falloff "/Game/ElementalDamage/Fire/DTBP_Fire.DTBP_Fire_C" _array DamageCauser InstigatedBy)
      (`AISense_Hearing.ReportNoiseEvent` _returnvalue 1.0 null)
      (`NiagaraFunctionLibrary.SpawnSystemAtLocation` "/Game/Effects/InfinityBladeEffects/Effects/FX_Monsters/FX_Monster_Gruntling/FlameThrower/P_FlameExplode_Converted.P_FlameExplode_Converted" _returnvalue)
      (`GameplayStatics.PlaySoundAtLocation` "/Game/Audio/Sounds/Explosions/Explosions_Grenade_Noise-Interior-Distant_01.Explosions_Grenade_Noise-Interior-Distant_01" _returnvalue (struct) 1.0 1.0 0.0 null null null null)
      (`self.K2_DestroyActor`))))

(fn `UserConstructionScript`
  (`parent.UserConstructionScript`))