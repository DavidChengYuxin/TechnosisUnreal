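; Base Blueprint for grabbable props that swaps the mesh to a dithered look during an interaction.
; The construction script sets the interactable component's type and builds MM_Dither-based copies of the mesh materials with transferred textures and a fixed alpha threshold.
; The Interact event switches every material slot between these copies and the cached originals as interaction starts or ends.
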(event `self.ReceiveBeginPlay`)

(event `/Game/Universal/Interact/BPI_Interact.Interact`
  (params (`InteractStart?` :type Boolean))
  (`self.SetMaterial` (select `bool` `InteractStart?` :`false` (`self.Original Materials`) :`true` (`self.Transfer Materials`) :!type "Array of MaterialInterface Object Reference")))

(fn `SetMaterial`
  (params (Materials :type "Array of MaterialInterface Object Reference"))
  (for (_array_element _array_index) Materials
    (`PrimitiveComponent.SetMaterial` (`self.Mesh`) _array_index _array_element)))

(fn `UserConstructionScript`
  (set `/Game/Universal/Interact/BPC_Interactable.InteractionType` "NewEnumerator2" (`self.BPC_Interactable`))
  (bind (_originalmaterials _transfermaterials) (`/Game/Universal/BPFL_Universal.TransferMeshTextures` (`self.Mesh`) "/Game/Universal/MasterMaterials/MM_Dither.MM_Dither"))
  (set `self.Original Materials` _originalmaterials)
  (bind _output_get (set `self.Transfer Materials` _transfermaterials))
  (for _array_element _output_get
    (`MaterialInstanceDynamic.SetScalarParameterValue` _array_element "AlphaThreshold" 0.333))
  (`self.SetMaterial` (`self.Original Materials`)))