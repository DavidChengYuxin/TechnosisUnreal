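; BP_OilPuddle is an oil puddle actor in the fire elemental damage system that burns when it takes fire damage.
; Its FireDamage event passes BurnDuration to the BPCFlammable component to add burn time.
; The construction script sets that component to destroy the puddle once it stops burning.
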(event `self.Fire Damage`
  (`/Game/ElementalDamage/Fire/BPC_Flammable.Event Add Burn Duration` (`self.BPC_Flammable`) (`self.BurnDuration`)))

(fn `UserConstructionScript`
  (`parent.UserConstructionScript`)
  (set `/Game/ElementalDamage/Fire/BPC_Flammable.DestroyOwnerOnStopBurning?` true (`self.BPC_Flammable`)))