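; Actor component that lets its owner catch fire, burn and spread fire to nearby actors.
; Fire-element damage extends burn duration unless BPC_Wettable is wet, enabling overlay, particles and AI status effect.
; A looping timer deals untyped self-damage to avoid re-igniting, and sphere-traces a scale-adjusted radius to apply fire damage.
; Burning ends on expiry, certain other elements or BPC_Health death, optionally destroying the owner; blackening is unfinished.
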(event `self.ReceiveBeginPlay`
  (bind _returnvalue (`Actor.GetComponentByClass` (`self.Owner`) "/Game/Universal/BPC_Health.BPC_Health_C"))
  (bind _output_get (set `self.Owner` (`self.GetOwner`)))
  (`|ExecutionSequence`
    (:`then_0`
      (bind _meshcompoments (`/Game/Universal/BPFL_Universal.Get All Mesh Components` _output_get))
      (bind _output_get_2 (set `self.Mesh Compoments` _meshcompoments))
      (for _ _output_get_2
        _))
    (:`then_1`
      (add `Actor.OnTakeAnyDamage` (`self.Owner`) (delegate `Event Owner Take Damage`)))
    (:`then_2`
      (bind _output_get_3 (set `self.OwnerImplementsHealthComponent?` (`KismetSystemLibrary.IsValid` _returnvalue)))
      (if _output_get_3
        (add `/Game/Universal/BPC_Health.DeathDispatcher` _returnvalue (delegate `Event Owner Dies`))))))

(event `Event Add Burn Duration`
  (params (AddSeconds :type "Float (double-precision)"))
  (set `self.Burn Duration` (+ (`self.Burn Duration`) AddSeconds))
  ;[1 1 1] Start burning if not already burning
  (if (not (`self.Burning?`))
    (`self.Event Start Burning`)))

(event `Event Owner Dies`
  ;[1 1 1] If owner has health, stop burning when dead
  (`self.Event Stop Burning`)
  (`self.Event Blacken Dead Owner`)
  (`self.K2_DestroyComponent`))

(event `EventBurnProximity`
  (params (OverlappedComponent :type "PrimitiveComponent Object Reference") (OtherActor :type "Actor Object Reference") (OtherComp :type "PrimitiveComponent Object Reference") (OtherBodyIndex :type Integer) (bFromSweep :type Boolean) (SweepResult :type "HitResult Structure (by ref)"))
  (bind _returnvalue (`self.GetOwner`))
  ;[1 1 1] Depreciated
  ;;[1 1 1] Applies burning to nearby actors
  (`GameplayStatics.ApplyDamage` OtherActor (`self.SpreadDamage`) (`Pawn.GetController` (`Actor.Instigator` _returnvalue)) _returnvalue "/Game/ElementalDamage/Fire/DTBP_Fire.DTBP_Fire_C"))

(event `Event Blacken Dead Owner`
  ;[1 1 1] WIP
  (for _array_element (`self.Mesh Compoments`)
    _))

(event `Event Owner Take Damage`
  (params (DamagedActor :type "Actor Object Reference") (Damage :type "Float (single-precision)") (DamageType :type "DamageType Object Reference") (InstigatedBy :type "Controller Object Reference") (DamageCauser :type "Actor Object Reference"))
  (bind _returnvalue (`Actor.GetComponentByClass` (`self.Owner`) "/Game/ElementalDamage/Water/BPC_Wettable.BPC_Wettable_C"))
  ;[1 1 1] When Owner recieves fire damage
  (if (`KismetSystemLibrary.DoesImplementInterface` DamageType "/Game/ElementalDamage/BPI_Element.BPI_Element_C")
    (bind _element (message `/Game/ElementalDamage/BPI_Element.GetElement` DamageType))
    (if (`|EnumEquality` _element "NewEnumerator1")
      (if (not (and (`KismetSystemLibrary.IsValid` _returnvalue) (`/Game/ElementalDamage/Water/BPC_Wettable.Wet?` _returnvalue)))
        (`self.Event Add Burn Duration` Damage)
        (if (not (`self.Burning?`))
          (`self.Event Start Burning`)))
      (elif (or (`|EnumEquality` _element "NewEnumerator6") (`|EnumEquality` _element "NewEnumerator3"))
        (`self.Event Stop Burning`)))))

(event `Event Start Burning`
  (bind _mesh_compoments (`self.Mesh Compoments`))
  (bind _returnvalue (`AIBlueprintHelperLibrary.GetAIController` (`self.Owner`)))
  (set `self.Burning?` true)
  (bind _returnvalue_2 (`KismetSystemLibrary.K2_SetTimerDelegate` (delegate `Event Tick Damage`) (`self.DeltaTime`) true true))
  (set `self.BurnTimer` _returnvalue_2)
  (`/Game/Universal/BPFL_Universal.Set All Mesh Components Overlay Material` _mesh_compoments (`self.Overlay Material`))
  (bind _particlecomponents (`/Game/Universal/BPFL_Universal.Set All Mesh Components Attached Particle` _mesh_compoments (`self.System Template`)))
  (set `self.ParticleComponents` _particlecomponents)
  (if (`KismetSystemLibrary.IsValid` _returnvalue)
    (message `/Game/AI/BPI_AI.AddStatusEffect` _returnvalue (`self.StatusEffectName`))))

(event `Event Tick Damage`
  (bind _owner (`self.Owner`))
  (bind (_returnvalue_x _returnvalue_y _returnvalue_z) (`KismetMathLibrary.BreakVector` (`Actor.GetActorScale3D` (`self.Owner`))))
  (bind _returnvalue (`Actor.K2_GetActorLocation` _owner))
  ;[1 1 1] Avoid infinite loop, don't set damage type to DTBP_Fire
  (`GameplayStatics.ApplyDamage` (`self.GetOwner`) (* (`self.DPS`) (`self.DeltaTime`)))
  (bind _output_get (set `self.Burn Duration` (- (`self.Burn Duration`) (`self.DeltaTime`))))
  (bind _outhits (`KismetSystemLibrary.SphereTraceMulti` _returnvalue _returnvalue (* (`self.EffectRadius`) (+ _returnvalue_x _returnvalue_y _returnvalue_z) 0.333333) "TraceTypeQuery2" false (`|MakeArray` _owner)))
  (for _array_element _outhits
    (`GameplayStatics.ApplyDamage` (`.HitActor` (`GameplayStatics.BreakHitResult` _array_element)) (`self.SpreadDamage`) null (`self.Owner`) "/Game/ElementalDamage/Fire/DTBP_Fire.DTBP_Fire_C"))
  (if (<= _output_get 0.0)
    (`self.Event Stop Burning`)))

(event `Event Stop Burning`
  (bind _returnvalue (`AIBlueprintHelperLibrary.GetAIController` (`self.Owner`)))
  (`|ExecutionSequence`
    (:`then_0`
      (set `self.Burning?` false)
      (`KismetSystemLibrary.K2_ClearAndInvalidateTimerHandle` (`self.BurnTimer`))
      (set `self.Burn Duration` 0.0))
    (:`then_1`
      ;[1 1 1] Remove effects
      (`/Game/Universal/BPFL_Universal.Set All Mesh Components Overlay Material` (`self.Mesh Compoments`) null false)
      (for _array_element (`self.ParticleComponents`)
        (`self.Deactivate` _array_element)))
    (:`then_2`
      ;[1 1 1] Destroys owner if Owner should be destroyed
      (if (`self.DestroyOwnerOnStopBurning?`)
        (`Actor.K2_DestroyActor` (`self.GetOwner`))))
    (:`then_3`
      (if (`KismetSystemLibrary.IsValid` _returnvalue)
        (message `/Game/AI/BPI_AI.RemoveStatusEffect` _returnvalue (`self.StatusEffectName`))))))

(fn `MinimumDamage`
  (params (MinimumDamage :type "Float (double-precision)"))
  (bind _returnvalue (- (`self.Burn Duration`) (`local.MinimumDamage`)))
  ;[1 1 1] Avoid infinite loop, don't set damage type to DTBP_Fire
  (`GameplayStatics.ApplyDamage` (`self.GetOwner`) MinimumDamage)
  (set `self.Burning?` false)
  (set `self.Burn Duration` (select `bool` (< _returnvalue 0.0) :`false` _returnvalue)))

(fn `Set Up Proximity`
  (params (Event :type "Delegate (by ref)"))
  (bind _returnvalue (`|AddComponentByClass` :`self` (`self.GetOwner`) :`Class` "/Script/Engine.SphereComponent"))
  (bind _output_get (set `self.EffectVolume` _returnvalue))
  (`SphereComponent.SetSphereRadius` _output_get (`self.EffectRadius`) true)
  (add `PrimitiveComponent.OnComponentBeginOverlap` (`self.EffectVolume`) Event))