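; An actor that emits continuous radial damage of a selectable element, including Heal and NonLethal, around its particle component.
; While active, Tick applies DPS scaled by delta time within DamageRadius, mapping Element to a damage type class.
; Start and stop events, bound to dispatchers on BeginPlay, toggle the Generating flag, actor ticking and the particle together.
; The initial Generating value decides whether it starts active.
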(event `self.ReceiveBeginPlay`
  (add `self.StartDamageDispatcher` (delegate `Event Start Damage`))
  (add `self.StopDamageDispatcher` (delegate `Event Stop Damage`))
  (if (`self.Generating?`)
    (`self.Event Start Damage`)
    (else
      (`self.Event Stop Damage`))))

(event `Event Start Damage`
  (bind _output_get (set `self.Generating?` true))
  (`self.SetActorTickEnabled` _output_get)
  (`ActorComponent.Activate` (`self.Particle`) false))

(event `Event Stop Damage`
  (bind _output_get (set `self.Generating?` false))
  (`self.SetActorTickEnabled` _output_get)
  (`ActorComponent.Deactivate` (`self.Particle`)))

(event `self.ReceiveTick`
  (params (DeltaSeconds :type "Float (single-precision)"))
  (`GameplayStatics.ApplyRadialDamage` :`BaseDamage` (* DeltaSeconds (`self.DPS`)) :`Origin` (`SceneComponent.K2_GetComponentLocation` (`self.Particle`)) :`DamageRadius` (`self.DamageRadius`) :`DamageTypeClass` (select `/Game/ElementalDamage/Enum_Element` (`self.Element`) :`NewEnumerator0` "/Game/ElementalDamage/Kinetic/DTBP_Kinetic.DTBP_Kinetic_C" :`NewEnumerator1` "/Game/ElementalDamage/Fire/DTBP_Fire.DTBP_Fire_C" :`NewEnumerator2` "/Game/ElementalDamage/Electricity/DTBP_Electricity.DTBP_Electricity_C" :`NewEnumerator3` "/Game/ElementalDamage/Ice/DTBP_Ice.DTBP_Ice_C" :`NewEnumerator6` "/Game/ElementalDamage/Water/DTBP_Water.DTBP_Water_C" :`NewEnumerator5` "/Game/ElementalDamage/Chemical/DTBP_Chemical.DTBP_Chemical_C" :`NewEnumerator8` "/Game/ElementalDamage/ArmorPiercing/DTBP_ArmorPiercing.DTBP_ArmorPiercing_C" :`NewEnumerator7` "/Game/ElementalDamage/KnockBack/DTBP_KnockBack.DTBP_KnockBack_C" :`NewEnumerator9` "/Game/ElementalDamage/Heal/DTBP_Heal.DTBP_Heal_C" :`NewEnumerator4` "/Game/ElementalDamage/Non-Lethal/DTBP_NonLethal.DTBP_NonLethal_C" :!type "DamageType Class Reference") :`DamageCauser` null :`InstigatedByController` null))

(fn `UserConstructionScript`)