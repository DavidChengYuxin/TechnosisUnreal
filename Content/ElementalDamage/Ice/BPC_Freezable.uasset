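; Actor component that lets its owner freeze under ice damage and thaw under fire damage.
; It binds to the owner's damage event, reads the element through BPI_Element, and accumulates ice damage until FrozenPercentage reaches one.
; Freezing applies an overlay material and attached particles to the owner's meshes, also pausing animation and disabling movement for Characters.
; Thawing reverses these effects but leaves FrozenPercentage unchanged.
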(event `self.ReceiveBeginPlay`
  (bind _output_get (set `self.Owner` (`self.GetOwner`)))
  (`|ExecutionSequence`
    (:`then_0`
      ;[1 1 1] Get character movement if owner is character, else set a flag that owner is not a character, and ignores any disabled movement
      (bind _ascharacter (cast `Character` _output_get)
        (:`then`
          (set `self.Character Movement` (`Character.CharacterMovement` _ascharacter)))
        (:`CastFailed`
          (set `self.OwnerIsCharacter?` false))))
    (:`then_1`
      ;[1 1 1] Get all components of Owner
      (bind _meshcompoments (`/Game/Universal/BPFL_Universal.Get All Mesh Components` null))
      (bind _output_get_2 (set `self.Mesh Compoments` _meshcompoments))
      (for _array_element _output_get_2
        (bind _asskeletal_mesh_component (cast `SkeletalMeshComponent` _array_element))
        (`KismetArrayLibrary.Array_Add` (`self.Skeletal Mesh Components`) _asskeletal_mesh_component)))
    (:`then_2`
      ;[1 1 1] Binds Owner's take damage event
      (add `Actor.OnTakeAnyDamage` (`self.Owner`) (delegate `Event Owner Take Damage`)))))

(event `Event Owner Take Damage`
  (params (DamagedActor :type "Actor Object Reference") (Damage :type "Float (single-precision)") (DamageType :type "DamageType Object Reference") (InstigatedBy :type "Controller Object Reference") (DamageCauser :type "Actor Object Reference"))
  ;[1 1 1] When Owner recieves ice damage
  (if (`KismetSystemLibrary.DoesImplementInterface` DamageType "/Game/ElementalDamage/BPI_Element.BPI_Element_C")
    (bind _element (message `/Game/ElementalDamage/BPI_Element.GetElement` DamageType))
    (if (`|EnumEquality` _element "NewEnumerator3")
      (bind _output_get (set `self.FrozenPercentage` (+ (`self.FrozenPercentage`) Damage)))
      (if (>= _output_get 1.0)
        (`self.Event Freeze`))
      (else
        ;[1 1 1] Melts Owner if fire damage recieved
        (if (`|EnumEquality` _element "NewEnumerator1")
          (`self.Event Unfreeze`))))))

(event `Event Freeze`
  (bind _mesh_compoments (`self.Mesh Compoments`))
  (if (not (`self.Frozen?`))
    (set `self.Frozen?` true)
    (`self.FreezeCharacter`)
    (`/Game/Universal/BPFL_Universal.Set All Mesh Components Overlay Material` _mesh_compoments (`self.Overlay Material`))
    (bind _particlecomponents (`/Game/Universal/BPFL_Universal.Set All Mesh Components Attached Particle` _mesh_compoments (`self.System Template`)))
    (set `self.ParticleComponents` _particlecomponents)))

(event `Event Unfreeze`
  (set `self.Frozen?` false)
  (`self.Unfreeze Character`)
  (`/Game/Universal/BPFL_Universal.Set All Mesh Components Overlay Material` (`self.Mesh Compoments`) null false)
  (for _array_element (`self.ParticleComponents`)
    (`self.K2_DestroyComponent` _array_element)))

(fn `FreezeCharacter`
  (if (`self.OwnerIsCharacter?`)
    (`|ExecutionSequence`
      (:`then_0`
        (for _array_element (`self.Skeletal Mesh Components`)
          (set `SkeletalMeshComponent.bPauseAnims` true _array_element)))
      (:`then_1`
        (`CharacterMovementComponent.DisableMovement` (`self.Character Movement`))))))

(fn `Unfreeze Character`
  (if (`self.OwnerIsCharacter?`)
    (`|ExecutionSequence`
      (:`then_0`
        (for _array_element (`self.Skeletal Mesh Components`)
          (set `SkeletalMeshComponent.bPauseAnims` false _array_element)))
      (:`then_1`
        (`CharacterMovementComponent.SetMovementMode` (`self.Character Movement`) "MOVE_Walking" 0)))))