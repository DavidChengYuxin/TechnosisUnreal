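; Elemental ice puddle hazard that deals token knockback-type damage to any actor that begins overlapping it.
; On BeginPlay it sets a timeline to its lifetime duration, and timeline completion calls Transmute to turn it into another elemental form.
; Ice damage restarts that countdown, while fire damage destroys the puddle immediately.
; A deprecated, disconnected LaunchCharacter branch remains in the graph.
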(event `self.ReceiveBeginPlay`
  (`parent.ReceiveBeginPlay`)
  (`TimelineComponent.SetTimelineLength` (`self.TimelineToDestroy`) (`self.LifetimeDuration`))
  (`Timeline|Timeline` :!via `PlayFromStart`
    (:`Finished`
      (`self.Transmute` "NewEnumerator6"))))

(event `self.ReceiveActorBeginOverlap`
  (params (OtherActor :type "Actor Object Reference"))
  (`parent.ReceiveActorBeginOverlap` OtherActor)
  (`GameplayStatics.ApplyDamage` OtherActor 1.0 null null "/Game/ElementalDamage/KnockBack/DTBP_KnockBack.DTBP_KnockBack_C"))

(event `self.Ice Damage`
  ;[1 1 1] Resets timer to freeze
  (`Timeline|TimelineToDestroy` :!via `PlayFromStart`
    (:`Finished`
      (`self.Transmute` "NewEnumerator6"))))

(event `self.Fire Damage`
  (`self.K2_DestroyActor`))

(fn `UserConstructionScript`
  (`parent.UserConstructionScript`))