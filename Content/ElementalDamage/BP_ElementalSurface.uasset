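; Base actor for elemental surfaces such as puddles, which react to elemental damage and can transmute into other surface types.
; AnyDamage reads the element from the damage type through BPI_Element and routes it to empty per-element events, apparently meant for child overrides.
; Transmute spawns the selected surface class and particle system at its transform, credits the damage instigator, then destroys itself.
; Destruction triggers a decal fade-out; the default element is Kinetic.
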(event `self.ReceiveAnyDamage`
  (params (Damage :type "Float (single-precision)") (DamageType :type "DamageType Object Reference") (InstigatedBy :type "Controller Object Reference") (DamageCauser :type "Actor Object Reference"))
  (set `self.Instigated By` InstigatedBy)
  (if (`KismetSystemLibrary.DoesImplementInterface` DamageType "/Game/ElementalDamage/BPI_Element.BPI_Element_C")
    (bind _element (message `/Game/ElementalDamage/BPI_Element.GetElement` DamageType))
    (switch `/Game/ElementalDamage/Enum_Element` _element
      (:`NewEnumerator1`
        (`self.Fire Damage`))
      (:`NewEnumerator2`
        (`self.Electricity Damage`))
      (:`NewEnumerator3`
        (`self.Ice Damage`))
      (:`NewEnumerator6`
        (`self.Water Damage`))
      (:`NewEnumerator5`
        (`self.Chemical Damage`)))))

(event `Fire Damage`)

(event `Electricity Damage`)

(event `Ice Damage`)

(event `Water Damage`)

(event `Chemical Damage`)

(event `Transmute`
  (params (Selection :type "/Game/ElementalDamage/Enum_Element Enum" :default "NewEnumerator0"))
  (bind (_returnvalue_location _returnvalue_rotation _returnvalue_scale) (`KismetMathLibrary.BreakTransform` (`self.GetTransform`)))
  (`|SpawnActorFromClass` (select `/Game/ElementalDamage/Enum_Element` Selection :`NewEnumerator1` "/Game/ElementalDamage/Fire/BP_OilPuddle.BP_OilPuddle_C" :`NewEnumerator3` "/Game/ElementalDamage/Ice/BP_IcePuddle.BP_IcePuddle_C" :`NewEnumerator6` "/Game/ElementalDamage/Water/BP_WaterPuddle.BP_WaterPuddle_C" :`NewEnumerator5` "/Game/ElementalDamage/Chemical/BP_ChemicalPuddle.BP_ChemicalPuddle_C" :!type "Actor Class Reference") (`self.GetTransform`) "Undefined" "MultiplyWithRoot" null (`Controller.K2_GetPawn` (`self.Instigated By`)))
  (`NiagaraFunctionLibrary.SpawnSystemAtLocation` (select `/Game/ElementalDamage/Enum_Element` Selection :!type "NiagaraSystem Object Reference") _returnvalue_location _returnvalue_rotation _returnvalue_scale)
  (`self.K2_DestroyActor`))

(event `self.ReceiveDestroyed`
  (`self.DestroyDecalWithOwner`))

(fn `DestroyDecalWithOwner`
  (`DecalComponent.SetFadeOut` (`self.Decal`) 0.0 (`self.FadeOutDuration`) true))

(fn `GetElement`
  (returns (Element :type "/Game/ElementalDamage/Enum_Element Enum"))
  (return "NewEnumerator0"))

(fn `UserConstructionScript`)