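; Water puddle actor for the elemental damage system that applies a small amount of water damage to actors that begin overlapping its box.
; At BeginPlay it hands that box to its conductive component as the proximity collider override.
; Ice and chemical damage each transmute the puddle into a different type, fire destroys it, and electricity attaches an electric-surface Niagara effect.
; Leftover nodes for setting the conductive radius and volume are unwired.
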(event `self.ReceiveBeginPlay`
  (`parent.ReceiveBeginPlay`)
  (`/Game/ElementalDamage/Electricity/BPC_Conductive.Event Override Proximity Collidor` (`self.BPC_Conductive`) (`self.Box`)))

(event `self.Ice Damage`
  (`self.Transmute` "NewEnumerator3"))

(event `self.Electricity Damage`
  (`NiagaraFunctionLibrary.SpawnSystemAttached` "/Game/Effects/ElementalDamage/Electric/NS_ElectricSurface.NS_ElectricSurface" (`self.DefaultSceneRoot`) "None" (0.0 0.0 0.0) (struct) "KeepRelativeOffset" true))

(event `self.Chemical Damage`
  (`self.Transmute` "NewEnumerator5"))

(event `self.Fire Damage`
  (`self.K2_DestroyActor`))

(event `self.Box.OnComponentBeginOverlap`
  (params (OverlappedComponent :type "PrimitiveComponent Object Reference") (OtherActor :type "Actor Object Reference") (OtherComp :type "PrimitiveComponent Object Reference") (OtherBodyIndex :type Integer) (bFromSweep :type Boolean) (SweepResult :type "HitResult Structure (by ref)"))
  (`GameplayStatics.ApplyDamage` OtherActor 0.5 null null "/Game/ElementalDamage/Water/DTBP_Water.DTBP_Water_C"))

(fn `UserConstructionScript`
  (`parent.UserConstructionScript`))