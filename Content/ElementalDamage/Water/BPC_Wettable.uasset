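; BPC_Wettable is an actor component that makes its owner wet from water damage, with damage scaled into a capped wetness duration.
; While wet, it applies an overlay material, stops burning, and temporarily adds freezable and conductive components if the owner lacked them at BeginPlay.
; Tick runs only while wet, counting the duration down unless submerged.
; Drying removes the overlay and added components; chemical-burn removal is unfinished.
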(event `self.ReceiveBeginPlay`
  (bind _owner (`self.Owner`))
  (bind _output_get (set `self.Owner` (`self.GetOwner`)))
  (`|ExecutionSequence`
    (:`then_0`
      (bind _meshcompoments (`/Game/Universal/BPFL_Universal.Get All Mesh Components` _output_get))
      (set `self.OwnerMeshComponents` _meshcompoments))
    (:`then_1`
      (`|ExecutionSequence`
        (:`then_0`
          (set `self.OwnerConductive?` (`KismetSystemLibrary.IsValid` (`Actor.GetComponentByClass` _owner "/Game/ElementalDamage/Electricity/BPC_Conductive.BPC_Conductive_C"))))
        (:`then_1`
          (set `self.OwnerFlammable` (`KismetSystemLibrary.IsValid` (`Actor.GetComponentByClass` _owner "/Game/ElementalDamage/Fire/BPC_Flammable.BPC_Flammable_C"))))
        (:`then_2`
          (set `self.OwnerFreezeable?` (`KismetSystemLibrary.IsValid` (`Actor.GetComponentByClass` _owner "/Game/ElementalDamage/Ice/BPC_Freezable.BPC_Freezable_C"))))))
    (:`then_2`
      ;[1 1 1] Sanity check. Tick should be disabled at start. But if wet, enable tick.
      (if (`self.Wet?`)
        (`self.SetComponentTickEnabled` true)))
    (:`then_3`
      (add `Actor.OnTakeAnyDamage` (`self.Owner`) (delegate `Event Owner Take Damage`)))))

(event `Event Owner Take Damage`
  (params (DamagedActor :type "Actor Object Reference") (Damage :type "Float (single-precision)") (DamageType :type "DamageType Object Reference") (InstigatedBy :type "Controller Object Reference") (DamageCauser :type "Actor Object Reference"))
  ;[1 1 1] When Owner recieves water damage
  (if (`KismetSystemLibrary.DoesImplementInterface` DamageType "/Game/ElementalDamage/BPI_Element.BPI_Element_C")
    (bind _element (message `/Game/ElementalDamage/BPI_Element.GetElement` DamageType))
    (if (`|EnumEquality` _element "NewEnumerator6")
      (`self.Event Add Wet Duration` (* (`self.DamageToDurationMultiplier`) Damage)))))

(event `self.ReceiveTick`
  (params (DeltaSeconds :type "Float (single-precision)"))
  ;[1 1 1] Sanity check. Tick should be disabled unless wet.
  (if (`self.Wet?`)
    (if (not (`self.Submerged?`))
      (`self.Event Subtract Wet Duration` DeltaSeconds))
    (else
      (`self.SetComponentTickEnabled` false))))

(event `Event Set Wet`
  (bind _output_get (set `self.Wet?` true))
  (`self.SetComponentTickEnabled` _output_get)
  (`/Game/Universal/BPFL_Universal.Set All Mesh Components Overlay Material` (`self.OwnerMeshComponents`) (`self.Overlay Material`))
  (`|ExecutionSequence`
    (:`then_0`
      ;[1 1 1] Makes owner temporarily freezeable (no change if owner is already freezeable)
      (if (not (`self.OwnerFreezeable?`))
        (`|AddComponentByClass` (`self.Owner`) "/Game/ElementalDamage/Ice/BPC_Freezable.BPC_Freezable_C")))
    (:`then_1`
      ;[1 1 1] Makes owner temporarily conductive (no change if owner is already freezeable)
      (if (not (`self.OwnerConductive?`))
        (`|AddComponentByClass` (`self.Owner`) "/Game/ElementalDamage/Electricity/BPC_Conductive.BPC_Conductive_C")))
    (:`then_2`
      ;[1 1 1] Stops burning
      (if (`self.OwnerFlammable`)
        (`/Game/ElementalDamage/Fire/BPC_Flammable.Event Stop Burning` (`Actor.GetComponentByClass` (`self.Owner`) "/Game/ElementalDamage/Fire/BPC_Flammable.BPC_Flammable_C"))))
    (:`then_3`
      ;[1 1 1] Stops chemical burn (WORK IN PROGRESS)
      (if true
        _))))

(event `Event Add Wet Duration`
  (params (AddSeconds :type "Float (double-precision)"))
  ;[1 1 1] Add and remove wetness duration
  (bind _output_get (set `self.WetDuration` (`KismetMathLibrary.FClamp` (+ AddSeconds (`self.WetDuration`)) 0.0 (`self.MaxWetDuration`))))
  (if (and (not (`self.Wet?`)) (> _output_get 0.0))
    (`self.Event Set Wet`)))

(event `Event Subtract Wet Duration`
  (params (SubtractSeconds :type "Float (double-precision)"))
  ;[1 1 1] Add and remove wetness duration
  (if (not (`self.Submerged?`))
    (bind _output_get (set `self.WetDuration` (`KismetMathLibrary.FClamp` (- (`self.WetDuration`) SubtractSeconds) 0.0 (`self.MaxWetDuration`))))
    (if (<= _output_get 0.0)
      (`self.Event Set Dry`))))

(event `Event Set Dry`
  (bind _output_get (set `self.Wet?` false))
  (`self.SetComponentTickEnabled` _output_get)
  (`/Game/Universal/BPFL_Universal.Set All Mesh Components Overlay Material` (`self.OwnerMeshComponents`) null false)
  ;[1 1 1] Removes freezeability (iff actor was previous unfreezeable)
  (if (not (`self.OwnerFreezeable?`))
    (`self.K2_DestroyComponent` (`Actor.GetComponentByClass` (`self.Owner`) "/Game/ElementalDamage/Ice/BPC_Freezable.BPC_Freezable_C") (`self.Owner`)))
  ;[1 1 1] Remove conductiveness (iff actor was previously non-conductive)
  (if (not (`self.OwnerConductive?`))
    (`self.K2_DestroyComponent` (`Actor.GetComponentByClass` (`self.GetOwner`) "/Game/ElementalDamage/Electricity/BPC_Conductive.BPC_Conductive_C"))))

(fn `GetOwnerMeshes`)