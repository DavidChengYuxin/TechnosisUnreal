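; Actor component that makes its owner electrocutable, reacting to electric damage with visual, audio and AI status effects.
; On any damage, it checks the damage type's element through BPI_Element to trigger electrocution.
; Electrocution overlays a material on cached meshes, plays a sound and starts a short timer that repeated hits restart.
; A DoOnce adds the AI controller status effect once until the timer clears everything.
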(event `self.ReceiveBeginPlay`
  (bind _output_get (set `self.Owner` (`self.GetOwner`)))
  (`|ExecutionSequence`
    (:`then_0`
      (bind _meshcompoments (`/Game/Universal/BPFL_Universal.Get All Mesh Components` _output_get))
      (set `self.Mesh Compoments` _meshcompoments))
    (:`then_1`
      (add `Actor.OnTakeAnyDamage` (`self.Owner`) (delegate `Event Owner Takes Damage`)))))

(event `Event Owner Takes Damage`
  (params (DamagedActor :type "Actor Object Reference") (Damage :type "Float (single-precision)") (DamageType :type "DamageType Object Reference") (InstigatedBy :type "Controller Object Reference") (DamageCauser :type "Actor Object Reference"))
  (if (`KismetSystemLibrary.DoesImplementInterface` DamageType "/Game/ElementalDamage/BPI_Element.BPI_Element_C")
    (bind _element (message `/Game/ElementalDamage/BPI_Element.GetElement` DamageType))
    (if (`|EnumEquality` _element "NewEnumerator2")
      (`self.Event Start Electrocuted`))))

(event `Event Start Electrocuted`
  (`|ExecutionSequence`
    (:`then_0`
      (`/Game/Universal/BPFL_Universal.Set All Mesh Components Overlay Material` (`self.Mesh Compoments`) (`self.Overlay Material`)))
    (:`then_1`
      (`GameplayStatics.PlaySoundAtLocation` "/Game/SoundEffects/FreeSound/jeremysykes/341666__jeremysykes__electricity00.341666__jeremysykes__electricity00" (`Actor.K2_GetActorLocation` (`self.Owner`)) (struct) 1.0 1.0 0.0 "/Game/Audio/AttenuationPresets/ATT_Default.ATT_Default" null null null))
    (:`then_2`
      (bind _returnvalue (`KismetSystemLibrary.K2_SetTimerDelegate` (delegate `Event Stop Electrocuted`) 0.3 false true))
      (set `self.ElectrocutionTimer` _returnvalue))
    (:`then_3`
      (`/Engine/EditorBlueprintResources/StandardMacros.DoOnce` false :!label _label
        (:`Completed`
          (message `/Game/AI/BPI_AI.AddStatusEffect` (`AIBlueprintHelperLibrary.GetAIController` (`self.Owner`)) (`self.StatusEffectName`)))))))

(event `Event Stop Electrocuted`
  (`|ExecutionSequence`
    (:`then_0`
      (`/Game/Universal/BPFL_Universal.Set All Mesh Components Overlay Material` (`self.Mesh Compoments`) null false))
    (:`then_1`
      (goto _label :!via `Reset`))
    (:`then_2`
      (message `/Game/AI/BPI_AI.RemoveStatusEffect` (`AIBlueprintHelperLibrary.GetAIController` (`self.Owner`)) (`self.StatusEffectName`)))
    (:`then_3`
      (`KismetSystemLibrary.K2_ClearAndInvalidateTimerHandle` (`self.ElectrocutionTimer`)))))