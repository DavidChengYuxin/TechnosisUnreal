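; Cigarette utility equipment that damages its holder and anyone caught in its second-hand smoke.
; On trigger start it applies fire-type damage to the parent actor, then to every hit from an upward sphere trace at the mesh, passing the smoke fire duration as the damage amount.
; Without a parent actor, construction makes it a physics-simulated object with an interactable component for grabbing.
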(event `/Game/Equipment/BPI_Equipment.Trigger`
  (params (`Start?` :type Boolean))
  (bind _parentactor (`self.ParentActor`))
  (bind _parentactor_2 (`self.ParentActor`))
  (bind _returnvalue (`SceneComponent.K2_GetComponentLocation` (`self.Mesh`)))
  (if `Start?`
    ;[1 1 1] Self-inflicted damage from smoking (include chemical damage as well?)
    (`GameplayStatics.ApplyDamage` _parentactor (`self.SmokeFireDuration`) (`self.GetInstigatorController` _parentactor) _parentactor "/Game/ElementalDamage/Fire/DTBP_Fire.DTBP_Fire_C")
    ;[1 1 1] 2nd Hand smoke
    (bind _outhits (`KismetSystemLibrary.SphereTraceMulti` _returnvalue (+ _returnvalue (* (`KismetMathLibrary.Vector_Up`) (`self.SmokeMaximumHeight`))) (`self.SmokeRadius`) "TraceTypeQuery1"))
    (for _array_element _outhits
      (`GameplayStatics.ApplyDamage` (`.HitActor` (`GameplayStatics.BreakHitResult` _array_element)) (`self.SmokeFireDuration`) (`self.GetInstigatorController` _parentactor_2) _parentactor_2 "/Game/ElementalDamage/Fire/DTBP_Fire.DTBP_Fire_C"))))

(event `/Game/Equipment/BPI_Equipment.Alt`
  (params (`Start?` :type Boolean)))

(fn `SetAsPhysicsObject`
  (bind _mesh (`self.Mesh`))
  (`PrimitiveComponent.SetCollisionProfileName` _mesh "BlockAll" false)
  (`PrimitiveComponent.SetSimulatePhysics` _mesh true))

(fn `UserConstructionScript`
  (bind _returnvalue (`self.GetParentActor`))
  (`/Engine/EditorBlueprintResources/StandardMacros.IsValid` _returnvalue
    (:`Is Valid`
      (set `self.ParentActor` _returnvalue))
    (:`Is Not Valid`
      ;[1 1 1] If no parent, assume to be grabbable object
      (`self.SetAsPhysicsObject`)
      ;[1 1 1] Make grabbable
      (bind _returnvalue_2 (`AddComponent|NODE_AddBPC_Interactable-0`))
      (set `/Game/Universal/Interact/BPC_Interactable.InteractionType` "NewEnumerator4" _returnvalue_2))))