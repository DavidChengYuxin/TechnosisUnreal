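; Base weapon for the player and NPCs, attached as a child actor, or a physics object when parentless.
; Trigger drives single, burst or full-auto fire, using looping timers for repeat attacks.
; Each attack spawns effects, reports AI noise unless silenced, then fires a projectile from the muzzle arrow or line-traces from the owner's camera or eyeline.
; Hitscan applies elemental damage with per-bone multipliers.
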(event `/Game/Equipment/BPI_Equipment.Trigger`
  (params (`Start?` :type Boolean))
  (bind _output_get (set `self.Triggered?` `Start?`))
  (if _output_get
    ;[1 1 1] Start triggered
    (switch `/Game/Equipment/Weapons/Enum_WeaponMode` (`self.WeaponMode`)
      (:`NewEnumerator0`
        (`/Engine/EditorBlueprintResources/StandardMacros.DoOnce` false :!label _label
          (:`Completed`
            (`self.SingleAttack`))))
      (:`NewEnumerator1`
        (`/Engine/EditorBlueprintResources/StandardMacros.DoOnce` false :!label _label_2
          (:`Completed`
            (bind _returnvalue (`KismetSystemLibrary.K2_SetTimerDelegate` (delegate `Event Burst`) (`self.HitDelay`) true true))
            (set `self.BurstTimerHandle` _returnvalue)
            (`self.Event Burst`))))
      (:`NewEnumerator2`
        (bind _returnvalue_2 (`KismetSystemLibrary.K2_SetTimerDelegate` (delegate `Event Automatic`) (`self.HitDelay`) true true))
        (`self.Event Automatic`)))
    (else
      ;[1 1 1] Stop triggered
      (switch `/Game/Equipment/Weapons/Enum_WeaponMode` (`self.WeaponMode`)
        (:`NewEnumerator0`
          (goto _label :!via `Reset`))
        (:`NewEnumerator1`
          (goto _label_2 :!via `Reset`))
        (:`NewEnumerator2`
          (`KismetSystemLibrary.K2_ClearAndInvalidateTimerHandle` _returnvalue_2))))))

(event `Event Burst`
  (bind _burstcounter (`self.BurstCounter`))
  (`self.SingleAttack`)
  (`/Engine/EditorBlueprintResources/StandardMacros.IncrementInt` _burstcounter
    (:`  `
      (if (>= _burstcounter (`self.HitsPerBurst`))
        (`KismetSystemLibrary.K2_ClearAndInvalidateTimerHandle` (`self.BurstTimerHandle`))
        (set `self.BurstCounter` 0)))))

(event `Event Automatic`
  (`self.SingleAttack`))

(fn `Impact Sound And Decal`
  (params (ImpactDecal :type "MaterialInterface Object Reference") (ImpactSound :type "SoundBase Object Reference") (ImpactLocation :type "Vector Structure") (ImpactNormal :type "Vector Structure"))
  (locals (DecalSize :type "Float (double-precision)" :default 1.0) (DecalDuration :type "Float (double-precision)" :default 30.0) (SoundLoudness :type "Float (double-precision)" :default 0.2) (SoundRange :type "Float (double-precision)" :default 500.0))
  (`GameplayStatics.SpawnDecalAtLocation` ImpactDecal (`KismetMathLibrary.Conv_DoubleToVector` (`local.DecalSize`)) ImpactLocation (`KismetMathLibrary.Conv_VectorToRotator` ImpactNormal) (`local.DecalDuration`))
  (`self.Spawn Particle & Sound` null ImpactSound ImpactLocation (struct) (`local.SoundLoudness`) (`local.SoundRange`)))

(fn `SingleAttack`
  (locals (Projectile :type "Actor Class Reference"))
  (bind _returnvalue (`self.GetParentActor`))
  (bind (_start _end) (`self.CharacterHitScanVectors` 0.0))
  (bind (_returnvalue_location _returnvalue_rotation) (`KismetMathLibrary.BreakTransform` (`SceneComponent.K2_GetComponentToWorld` (`self.Arrow`))))
  (`self.Spawn Particle & Sound` (`self.AttackParticle`) (`self.AttackSound`) _returnvalue_location _returnvalue_rotation 1.0 (`self.AttackSoundRange`))
  (switch `/Game/Equipment/Weapons/Enum_AttackMethod` (`self.AttackMethod`)
    (:`NewEnumerator0`
      (if true
        (bind (_outhit _returnvalue_2) (`KismetSystemLibrary.LineTraceSingle` _start _end "TraceTypeQuery1" false (`|MakeArray` (`self.ParentActor`)) "ForOneFrame"))
        (if _returnvalue_2
          (bind (_bblockinghit _binitialoverlap _time _distance _location _impactpoint _normal _impactnormal _physmat _hitactor _hitcomponent _hitbonename) (`GameplayStatics.BreakHitResult` _outhit))
          (`/Engine/EditorBlueprintResources/StandardMacros.IsValid` _hitactor
            (:`Is Valid`
              (bind (_value _returnvalue_3) (`BlueprintMapLibrary.Map_Find` (`self.PerBoneDamageMultiplier`) _hitbonename))
              (`GameplayStatics.ApplyDamage` _hitactor (* (`self.DamagePerHit`) (select `bool` _returnvalue_3 :`false` 1.0 :`true` _value)) (`self.GetInstigatorController` _returnvalue) _returnvalue (`/Game/Universal/BDML_Universal.GetElementalDamageClass` (`self.WeaponElement`))))
            (:`Is Not Valid`
              (`self.Impact Sound And Decal` null null _impactpoint _impactnormal))))))
    (:`NewEnumerator1`
      (`|SpawnActorFromClass` (`local.Projectile`) (`SceneComponent.K2_GetComponentToWorld` (`self.Arrow`)) "Undefined" "MultiplyWithRoot" null null))))

(fn `Spawn Particle & Sound`
  (params (Particle :type "NiagaraSystem Object Reference") (Sound :type "SoundBase Object Reference") (Location :type "Vector Structure") (Rotation :type "Rotator Structure") (Loudness :type "Float (single-precision)") (MaxRange :type "Float (single-precision)"))
  (`NiagaraFunctionLibrary.SpawnSystemAtLocation` Particle Location Rotation)
  (`GameplayStatics.SpawnSoundAtLocation` Sound Location (struct) 1.0 1.0 0.0 null null)
  (if (not (`self.Silenced?`))
    (`AISense_Hearing.ReportNoiseEvent` Location Loudness (`self.GetInstigatorController` (`self.GetParentActor`)) MaxRange)))

(fn `UserConstructionScript`
  (bind _returnvalue (`self.GetParentActor`))
  (bind _mesh (`self.Mesh`))
  (`/Engine/EditorBlueprintResources/StandardMacros.IsValid` _returnvalue
    (:`Is Valid`
      (set `self.ParentActor` _returnvalue)
      ;[1 1 1] Sets reference object to Third Person character or NPC parent. In future, rewrite to remove dependancy (probably by calling in interface)
      (bind _asbp_player_character (cast `/Game/Player/Blueprints/BP_PlayerCharacter` _returnvalue)
        (:`then`
          (set `self.OwnerReferenceComponent` (`/Game/Player/Blueprints/BP_PlayerCharacter.1stPersonCamera` _asbp_player_character)))
        (:`CastFailed`
          (bind _asbp_npc_parent (cast `/Game/AI/BP_NPC_Parent` _returnvalue))
          (set `self.OwnerReferenceComponent` (`/Game/AI/BP_NPC_Parent.Eyeline` _asbp_npc_parent)))))
    (:`Is Not Valid`
      ;[1 1 1] WIP if No parent, assume to be grabbable object
      (`PrimitiveComponent.SetCollisionProfileName` _mesh "BlockAll" false)
      (`PrimitiveComponent.SetSimulatePhysics` _mesh true))))