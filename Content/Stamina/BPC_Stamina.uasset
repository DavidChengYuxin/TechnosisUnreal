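; Actor component that tracks charge-based stamina, handling consumption and delayed regeneration.
; ConsumeStamina subtracts the cost without clamping, restarts the recharge delay, halts regeneration and enables component tick.
; StaminaRegenTick counts the delay down, then raises Stamina at a constant rate toward the Charges maximum.
; Tick switches itself off once stamina is full, so it only runs during the delay and recharge.
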(event `self.ReceiveTick`
  (params (DeltaSeconds :type "Float (single-precision)"))
  (bind _charges (`self.Charges`))
  ;[1 1 1] Tick should only be enabled when stamina is recharging
  (if (`self.RegeneratingStamina?`)
    (set `self.Stamina` (`KismetMathLibrary.FInterpTo_Constant` (`self.Stamina`) (`KismetMathLibrary.Conv_IntToDouble` (`self.Charges`)) (`GameplayStatics.GetWorldDeltaSeconds`) (`self.StaminaRechargeRate`)))
    (if (not (< (`self.Stamina`) _charges))
      (set `self.Stamina` (`KismetMathLibrary.Conv_IntToDouble` _charges))
      (`self.SetComponentTickEnabled` false)
      (set `self.RegeneratingStamina?` false))
    (else
      (bind _output_get (set `self.RechargeCurrentDelay` (`KismetMathLibrary.FInterpTo_Constant` (`self.RechargeCurrentDelay`) 0.0 (`GameplayStatics.GetWorldDeltaSeconds`) 1.0)))
      (if (<= _output_get 0.0)
        (set `self.RegeneratingStamina?` true)))))

(fn `Consume Stamina`
  (params (Consumption :type "Float (double-precision)" :default 1.0))
  (set `self.Stamina` (- (`self.Stamina`) Consumption))
  (set `self.RechargeCurrentDelay` (`self.RechargeMaxDelayDuration`))
  (set `self.RegeneratingStamina?` false)
  (`self.SetComponentTickEnabled` true))