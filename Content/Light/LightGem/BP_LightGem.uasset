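; BP_LightGem is a light gem that measures the light reaching its parent actor to drive that actor's visibility.
; Each tick, it reads back a 4x4 scene capture render target and maps the brightest pixel's luminance to a rounded value on BPC_Visibility, which it adds if missing.
; While enabled, the parent's meshes are hidden from scene captures; disabling stops ticking and zeroes visibility.
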(event `self.ReceiveBeginPlay`
  (`self.BeginPlay`))

(event `self.ReceiveTick`
  (params (DeltaSeconds :type "Float (single-precision)"))
  (`self.SetVisibility`))

(fn `BeginPlay`
  (bind _returnvalue (`self.GetParentActor`))
  (bind _returnvalue_2 (`self.GetComponentByClass` _returnvalue "/Game/Universal/BPC_Visibility.BPC_Visibility_C"))
  (bind _returnvalue_3 (`KismetRenderingLibrary.CreateRenderTarget2D` 4 4))
  (bind _output_get (set `self.RenderTarget` _returnvalue_3))
  (set `SceneCaptureComponent2D.TextureTarget` _output_get (`self.SceneCaptureComponent2D`))
  (set `self.ParentMeshComponents` (`self.K2_GetComponentsByClass` _returnvalue "/Script/Engine.MeshComponent"))
  ;[1 1 1] Sanity Check
  (`/Engine/EditorBlueprintResources/StandardMacros.IsValid` _returnvalue_2
    (:`Is Valid`
      (set `self.ParentVisibilityComponent` _returnvalue_2))
    (:`Is Not Valid`
      (bind _returnvalue_4 (`|AddComponentByClass` (`self.GetParentActor`) "/Game/Universal/BPC_Visibility.BPC_Visibility_C"))
      (set `self.ParentVisibilityComponent` _returnvalue_4)))
  (`self.Enable or Disable Light Gem` true))

(fn `Enable or Disable Light Gem`
  (params (`Enable?` :type Boolean))
  (bind _output_get (set `self.Enabled?` `Enable?`))
  (`self.SetActorTickEnabled` _output_get)
  (for _array_element (`self.ParentMeshComponents`)
    (`PrimitiveComponent.SetHiddenInSceneCapture` _array_element _output_get)
    ;[1 1 1] When Light Gem is disabled, assume to be invisible (e.g., using invisibility)
    (if (not _output_get)
      (set `/Game/Universal/BPC_Visibility.Visibility` 0.0 (`self.ParentVisibilityComponent`)))))

(fn `ProcessLuminance`
  (set `/Game/Universal/BPC_Visibility.Visibility` (`/Game/Universal/BDML_Universal.RoundingFloat` (`KismetMathLibrary.MapRangeClamped` (`.MaxValue` (`KismetMathLibrary.MaxOfFloatArray` (`self.LuminanceArray`))) (`self.MinLuminace`) (`self.MaxLuminance`) 0.0 1.0) 1) (`self.ParentVisibilityComponent`)))

(fn `SetVisibility`
  (bind _outlinearsamples (`KismetRenderingLibrary.ReadRenderTargetRaw` (`self.RenderTarget`)))
  (for (_array_element _array_index) _outlinearsamples
    (`KismetArrayLibrary.Array_Set` (`self.LuminanceArray`) _array_index (`KismetMathLibrary.LinearColor_GetLuminance` _array_element)))
  (`self.ProcessLuminance`))

(fn `UserConstructionScript`)