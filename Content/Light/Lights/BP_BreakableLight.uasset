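; Breakable point or spot light actor that can be switched on and off and goes dark when damaged.
; Construction keeps the chosen light component, applies its settings and sizes attenuation from a forward line trace.
; A dynamic emissive material takes its colour and strength from the configured light values.
; Damage types implementing BPI_Element break it only if flagged in EffectedByElement; other damage always does.
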(event `/Game/Circuit/BPI_Circuitry.Switch`
  (params (`On?` :type Boolean))
  ;[1 1 1] If connected to circuit, turns on and off
  (`LightComponent.SetIntensity` (`self.Light`) (select `bool` `On?` :`true` (`self.Intensity`) :!type "Float (single-precision)"))
  (`self.SetMaterialLightIntensity` (`self.LightDynamicMaterial`)))

(event `self.ReceiveAnyDamage`
  (params (Damage :type "Float (single-precision)") (DamageType :type "DamageType Object Reference") (InstigatedBy :type "Controller Object Reference") (DamageCauser :type "Actor Object Reference"))
  ;[1 1 1] Breaks on any damage received. Subject to change
  (if (`KismetSystemLibrary.DoesImplementInterface` DamageType "/Game/ElementalDamage/BPI_Element.BPI_Element_C")
    (bind _element (message `/Game/ElementalDamage/BPI_Element.GetElement` DamageType))
    (bind (_value _returnvalue) (`BlueprintMapLibrary.Map_Find` (`self.EffectedByElement?`) _element))
    (if (and _value _returnvalue)
      (`self.Event Break`))
    (else
      (`self.Event Break`))))

(event `Event Break`
  ;[1 1 1] Breaks on any damage received. Subject to change
  (set `self.Unbroken?` false)
  (`LightComponent.SetIntensity` (`self.Light`) 0.0)
  (`self.SetMaterialLightIntensity` (`self.LightDynamicMaterial`)))

(fn `RecalculateAttenutationRadius`
  (bind _light (`self.Light`))
  (bind _returnvalue (`SceneComponent.K2_GetComponentLocation` _light))
  (bind (_outhit _returnvalue_2) (`KismetSystemLibrary.LineTraceSingle` _returnvalue (+ _returnvalue (* (`SceneComponent.GetForwardVector` _light) 5000.0)) "TraceTypeQuery1"))
  (if _returnvalue_2
    (switch `/Game/Light/Lights/Enum_LightType` (`self.Type`)
      (:`NewEnumerator0`
        (bind (_bblockinghit _binitialoverlap _time _distance) (`GameplayStatics.BreakHitResult` _outhit))
        (`LocalLightComponent.SetAttenuationRadius` (`self.PointLight`) (* _distance 2.0)))
      (:`NewEnumerator1`
        (`LocalLightComponent.SetAttenuationRadius` (`self.SpotLight`) (* _distance 1.414))))))

(fn `SetMaterialLightIntensity`
  (params (DynamicMaterial :type "MaterialInstanceDynamic Object Reference"))
  (locals (MaterialColour :type "LinearColor Structure"))
  (bind _output_get (set `local.MaterialColour` (`self.LightColour`)))
  (if (`self.UseTemperature?`)
    (`KismetMathLibrary.LinearColor_SetTemperature` _output_get (`self.Temperature`)))
  (`MaterialInstanceDynamic.SetVectorParameterValue` (`local.DynamicMaterial`) "Colour" (`local.MaterialColour`))
  (`MaterialInstanceDynamic.SetScalarParameterValue` (`local.DynamicMaterial`) "EmissiveStrength" (* (`self.Intensity`) 5e-05)))

(fn `UserConstructionScript`
  (bind _light (`self.Light`))
  (bind _spotlight (`self.SpotLight`))
  (bind _pointlight (`self.PointLight`))
  (set `self.Light` (select `/Game/Light/Lights/Enum_LightType` (`self.Type`) :`NewEnumerator0` (`self.PointLight`) :`NewEnumerator1` (`self.SpotLight`) :!type "PointLightComponent Object Reference"))
  (`ActorComponent.K2_DestroyComponent` (select `/Game/Light/Lights/Enum_LightType` (`self.Type`) :`NewEnumerator0` (`self.SpotLight`) :`NewEnumerator1` (`self.PointLight`) :!type "PointLightComponent Object Reference"))
  (`|ExecutionSequence`
    (:`then_0`
      (`LightComponent.SetIntensity` (`self.Light`) (`self.Intensity`)))
    (:`then_1`
      (`LightComponent.SetLightColor` _light (`self.LightColour`) true)
      (`LightComponent.SetUseTemperature` _light (`self.UseTemperature?`))
      (`LightComponent.SetTemperature` _light (`self.Temperature`)))
    (:`then_2`
      (switch `/Game/Light/Lights/Enum_LightType` (`self.Type`)
        (:`NewEnumerator0`
          (`PointLightComponent.SetSourceRadius` _pointlight (`self.SourceRadius`))
          (`PointLightComponent.SetSoftSourceRadius` _pointlight (`self.SoftSourceRadius`)))
        (:`NewEnumerator1`
          (`SpotLightComponent.SetOuterConeAngle` _spotlight (`self.InnerConeAngle`))
          (`SpotLightComponent.SetInnerConeAngle` _spotlight (`self.OuterConeAngle`))
          (`PointLightComponent.SetSourceRadius` _spotlight (`self.SourceRadius`))
          (`PointLightComponent.SetSoftSourceRadius` _spotlight (`self.SoftSourceRadius`)))))
    (:`then_3`
      (`self.RecalculateAttenutationRadius`))
    (:`then_4`
      (bind _returnvalue (`PrimitiveComponent.CreateDynamicMaterialInstance` (`self.Mesh`) 0 "/Game/Universal/MasterMaterials/MM_Emmisive.MM_Emmisive" "None"))
      (bind _output_get (set `self.LightDynamicMaterial` _returnvalue))
      (`self.SetMaterialLightIntensity` _output_get))))