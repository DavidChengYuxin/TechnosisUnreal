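; Toggle switch prop that controls linked objects in its Circuitry array.
; Interacting or calling PressButton flips the On state, sends it to each linked object through SwitchMessage, plays a 2D sound and runs a timeline that offsets the mesh vertically.
; Damage types implementing BPI_Element also press it when their element is Kinetic, Armor Piercing or Knock Back.
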(event `/Game/Universal/Interact/BPI_Interact.Interact`
  (params (`InteractStart?` :type Boolean) (Causer :type "Actor Object Reference") (Instigator :type "Controller Object Reference"))
  (if `InteractStart?`
    (`|ExecutionSequence` :!label _label
      (:`then_0`
        (set `self.On?` (not (`self.On?`))))
      (:`then_1`
        (for _array_element (`self.Circuitry`)
          (message `/Game/Circuit/BPI_Circuitry.Switch` _array_element (`self.On?`))))
      (:`then_2`
        (`GameplayStatics.PlaySound2D` (`self.Sound`) 1.0 1.0 0.0 null null))
      (:`then_3`
        (bind (_direction _height) (`Timeline|AnimationTimeline`)
          (:`Update`
            (`SceneComponent.K2_SetRelativeLocation` (`self.Mesh`) (`KismetMathLibrary.MakeVector` 0.0 0.0 (* _height 5.0)) false false)))))))

(event `Event Press Button`
  (goto _label))

(event `self.ReceiveAnyDamage`
  (params (Damage :type "Float (single-precision)") (DamageType :type "DamageType Object Reference") (InstigatedBy :type "Controller Object Reference") (DamageCauser :type "Actor Object Reference"))
  (if (`KismetSystemLibrary.DoesImplementInterface` DamageType "/Game/ElementalDamage/BPI_Element.BPI_Element_C")
    (bind _element (`/Game/Universal/BPFL_Universal.Get Element` DamageType))
    (switch `/Game/ElementalDamage/Enum_Element` _element
      (:`NewEnumerator0`
        _)
      (:`NewEnumerator8`
        _)
      (:`NewEnumerator7`
        _))
    (`self.Event Press Button`)))

(fn `UserConstructionScript`)