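; Double sliding door prop that moves two panels along their Y axis and plays sounds on opening and closing.
; Overridden fast and slow open events share the normal open, which plays a timeline lerping both panels between closed and open positions; closing reverses it.
; Damage types implementing BPI_Element are checked for the Explosive element, which destroys the door if it is flagged Destructible.
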(event `self.ReceiveAnyDamage`
  (params (Damage :type "Float (single-precision)") (DamageType :type "DamageType Object Reference") (InstigatedBy :type "Controller Object Reference") (DamageCauser :type "Actor Object Reference"))
  (if (`KismetSystemLibrary.DoesImplementInterface` DamageType "/Game/ElementalDamage/BPI_Element.BPI_Element_C")
    (bind _element (message `/Game/ElementalDamage/BPI_Element.GetElement` DamageType))
    (switch `/Game/ElementalDamage/Enum_Element` _element
      (:`NewEnumerator8`
        (if (`self.Destructible?`)
          (`self.K2_DestroyActor`))))))

(event `self.Event Open Fast`
  (params (`Closewise?` :type Boolean))
  ;[0.5 0.5 0.5] Override opening
  (`self.Event Open` :!label _label))

(event `self.Event Open`
  ;[0.5 0.5 0.5] Override opening
  (`GameplayStatics.PlaySoundAtLocation` (`self.OpenSlowSound`) (`SceneComponent.K2_GetComponentLocation` (`self.DefaultSceneRoot`)) (struct) 1.0 1.0 0.0 null null null null)
  (set `self.Open?` true)
  (bind (_direction _open) (`Timeline|Timeline` :!label _label_2)
    (:`Update`
      (`SceneComponent.K2_SetRelativeLocation` (`self.Door`) (`KismetMathLibrary.MakeVector` 125.0 (`KismetMathLibrary.Lerp` (`self.Door1CloseY`) (`self.Door1OpenY`) _open)) false false)
      (`SceneComponent.K2_SetRelativeLocation` (`self.2ndDoor`) (`KismetMathLibrary.MakeVector` 125.0 (`KismetMathLibrary.Lerp` (`self.Door2CloseY`) (`self.Door2OpenY`) _open)) false false))))

(event `self.Event Open Slow`
  (params (`Clockwise?` :type Boolean))
  ;[0.5 0.5 0.5] Override opening
  (goto _label))

(event `self.Event Close`
  ;[0.5 0.5 0.5] Override opening
  (`TimelineComponent.SetPlayRate` (`self.OpenTimeline`) 1.0)
  (`GameplayStatics.PlaySoundAtLocation` (`self.CloseSound`) (`SceneComponent.K2_GetComponentLocation` (`self.DefaultSceneRoot`)) (struct) 1.0 1.0 0.0 null null null null)
  (set `self.Open?` false)
  (goto _label_2 :!via `Reverse`))

(fn `UserConstructionScript`
  (`parent.UserConstructionScript`))