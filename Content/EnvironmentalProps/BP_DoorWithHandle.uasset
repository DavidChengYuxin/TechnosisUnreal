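; Interactable hinged door prop that supports locking, damage-driven forced opening and optional destruction.
; Interact toggles it; when locked, only actors with a matching key or allowed faction can open it.
; A timeline rotates the pivot away from or toward the closed pose, with direction based on the causer.
; Sufficient knockback damage slams it open even if locked, emitting AI noise and passing knockback damage to whatever it hits.
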(event `self.Interact`
  (params (`InteractStart?` :type Boolean) (Causer :type "Actor Object Reference") (Instigator :type "Controller Object Reference"))
  (`self.ProcessInteract` Causer))

(event `self.ReceiveAnyDamage`
  (params (Damage :type "Float (single-precision)") (DamageType :type "DamageType Object Reference") (InstigatedBy :type "Controller Object Reference") (DamageCauser :type "Actor Object Reference"))
  (bind _minimumknockbacktoopen (`self.MinimumKnockbackToOpen`))
  (`/Game/Universal/BPML_Universal.SwitchOnElementalDamage` DamageType
    (:`ArmorPiercing`
      (if (`self.Destructible?`)
        (`self.K2_DestroyActor`)))
    (:`KnockBack`
      (if (and (>= Damage _minimumknockbacktoopen) (> _minimumknockbacktoopen 0.0))
        (if (`self.Locked?`)
          (bind _openable_ (`self.Process Lock Strength`))
          (if _openable_
            (if (not (`self.Open?`)) :!label _label
              (`self.Event Open Fast` (`self.GetSwingOrientation` DamageCauser))
              (set `self.KnockbackInstigatedBy` InstigatedBy)))
          (else
            (goto _label)))))))

(event `Event Open Slow`
  (params (`Clockwise?` :type Boolean))
  ;[1 1 1] Open & Close Door
  (set `self.Clockwise?` `Clockwise?`)
  (`TimelineComponent.SetPlayRate` (`self.OpenTimeline`) 1.0)
  (`self.Event Open`))

(event `Event Open Fast`
  (params (`Closewise?` :type Boolean))
  (bind _location (`self.SoundLocation`))
  ;[1 1 1] Open & Close Door
  (set `self.Clockwise?` `Closewise?`)
  (`TimelineComponent.SetPlayRate` (`self.OpenTimeline`) 8.0)
  (`self.Event Open`)
  (set `self.Knockback?` true)
  (`GameplayStatics.PlaySoundAtLocation` (`self.OpenFastSound`) _location (struct) 1.0 1.0 0.0 null null null null)
  (`AISense_Hearing.ReportNoiseEvent` _location 1.0 (`self.KnockbackInstigatedBy`) 500.0))

(event `self.SetLock`
  (params (`Lock?` :type Boolean))
  (bind _open_ (`self.Open?`))
  (bind _output_get (set `self.Locked?` `Lock?`))
  (`|ExecutionSequence`
    (:`then_0`
      (if _output_get
        (if _open_
          (`self.Event Close`))
        (elif (not _open_)
          (`self.Event Open`))))
    (:`then_1`
      (set `/Game/Universal/Interact/BPC_Interactable.Interactable?` (not _output_get) (`self.BPC_Interactable`)))))

(event `Event Open`
  ;[1 1 1] Open & Close Door
  (`GameplayStatics.PlaySoundAtLocation` (`self.OpenSlowSound`) (`self.SoundLocation`) (struct) 1.0 1.0 0.0 null null null null)
  (set `self.Open?` true)
  (bind (_direction _open) (`Timeline|OpenTimeline` :!label _label_2)
    (:`Update`
      (`self.SetDoorRotation` _open (`self.Clockwise?`)))
    (:`Finished`
      (set `self.Knockback?` false))))

(event `self.ReceiveHit`
  (params (MyComp :type "PrimitiveComponent Object Reference") (Other :type "Actor Object Reference") (OtherComp :type "PrimitiveComponent Object Reference") (bSelfMoved :type Boolean) (HitLocation :type "Vector Structure") (HitNormal :type "Vector Structure") (NormalImpulse :type "Vector Structure") (Hit :type "HitResult Structure (by ref)"))
  (if (`self.Knockback?`)
    (`GameplayStatics.ApplyPointDamage` Other (`self.KnockbackMomentum`) HitLocation Hit (`self.KnockbackInstigatedBy`) self "/Game/ElementalDamage/KnockBack/DTBP_KnockBack.DTBP_KnockBack_C")))

(event `Event Close`
  ;[1 1 1] Open & Close Door
  (`TimelineComponent.SetPlayRate` (`self.OpenTimeline`) 1.0)
  (`GameplayStatics.PlaySoundAtLocation` (`self.CloseSound`) (`self.SoundLocation`) (struct) 1.0 1.0 0.0 null null null null)
  (set `self.Open?` false)
  (set `self.Knockback?` false)
  (goto _label_2 :!via `Reverse`))

(event `self.ReceiveDestroyed`
  (`NiagaraFunctionLibrary.SpawnSystemAtLocation` (`self.OnDestroyedParticle`))
  (`GameplayStatics.SpawnSoundAtLocation` (`self.OnDestroyedSound`) (0.0 0.0 0.0) (struct) 1.0 1.0 0.0 null null))

(fn `Process Lock Strength`
  (returns (`Openable?` :type Boolean))
  (return true))

(fn `ProcessInteract`
  (params (InteractionActor :type "Actor Object Reference"))
  (bind _returnvalue (`self.GetComponentByClass` (`local.InteractionActor`) "/Game/Items/BPC_Inventory.BPC_Inventory_C"))
  (bind _returnvalue_2 (`self.GetComponentByClass` (`local.InteractionActor`) "/Game/Universal/Factions/BPC_Faction.BPC_Faction_C"))
  (if (`self.Locked?`)
    ;[0.053 0.053 0.053] If instigator actor has key, open door.
    (`/Engine/EditorBlueprintResources/StandardMacros.IsValid` _returnvalue
      (:`Is Valid`
        (if (`/Game/Items/BPC_Inventory.HasKeyInArray?` _returnvalue (`self.Keys`))
          (`self.Event Open Slow` (`self.GetSwingOrientation` (`local.InteractionActor`)))
          (else
            ;[0.053 0.053 0.053] If instigator actor is a faction that can open, bypass locked door
            (`/Engine/EditorBlueprintResources/StandardMacros.IsValid` _returnvalue_2 :!label _label
              (:`Is Valid`
                (if (>= (`KismetArrayLibrary.Array_Find` (`self.FactionCanOpenLocked?`) (`/Game/Universal/Factions/BPC_Faction.Faction` _returnvalue_2)) 0)
                  (`self.Event Open Slow` (`self.GetSwingOrientation` (`local.InteractionActor`)))))
              (:`Is Not Valid`)))))
      (:`Is Not Valid`
        (goto _label)))
    (elif (`self.Open?`)
      (`self.Event Close`)
      (else
        (`self.Event Open Slow` (`self.GetSwingOrientation` InteractionActor))))))

(fn `SetDoorRotation`
  (params (Percent :type "Float (double-precision)") (`Clockwise?` :type Boolean))
  (bind _output_get (set `self.SwingPercent` Percent))
  (`SceneComponent.K2_SetRelativeRotation` (`self.Pivot`) (`KismetMathLibrary.MakeRotator` (* _output_get 90.0 (select `bool` `Clockwise?` :`false` 1.0 :`true` -1.0)) 90.0) false false))

(fn `UserConstructionScript`)