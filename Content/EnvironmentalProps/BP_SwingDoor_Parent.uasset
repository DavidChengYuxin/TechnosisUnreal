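; Parent Blueprint for a swinging door that opens and closes on interaction, with locked doors opening only for allowed factions.
; A timeline rotates the pivot up to 90 degrees, with play rate separating slow from fast opening.
; Elemental damage can destroy destructible doors (Explosive) or fling them open (Knock Back).
; Lock strength always passes, Unlock and SetLock are empty, and swing-orientation logic is unconnected.
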(event `/Game/Universal/Interact/BPI_Interact.Interact`
  (params (`InteractStart?` :type Boolean) (Causer :type "Actor Object Reference") (Instigator :type "Controller Object Reference"))
  (`self.InteractParent` Causer))

(event `self.ReceiveAnyDamage`
  (params (Damage :type "Float (single-precision)") (DamageType :type "DamageType Object Reference") (InstigatedBy :type "Controller Object Reference") (DamageCauser :type "Actor Object Reference"))
  (if (`KismetSystemLibrary.DoesImplementInterface` DamageType "/Game/ElementalDamage/BPI_Element.BPI_Element_C")
    (bind _element (message `/Game/ElementalDamage/BPI_Element.GetElement` DamageType))
    (switch `/Game/ElementalDamage/Enum_Element` _element
      (:`NewEnumerator8`
        (if (`self.Destructible?`)
          (`self.K2_DestroyActor`)))
      (:`NewEnumerator7`
        (if (`self.Locked?`)
          (bind _openable_ (`self.Process Lock Strength`))
          (if _openable_
            (if (not (`self.Open?`)) :!label _label
              (`self.Event Open Fast` (`self.GetSwingOrientation` DamageCauser))))
          (else
            (goto _label)))))))

(event `Event Open Slow`
  (params (`Clockwise?` :type Boolean))
  ;[1 1 1] Open & Close Door
  (set `self.Clockwise?` `Clockwise?`)
  (`TimelineComponent.SetPlayRate` (`self.OpenTimeline`) 1.0)
  (`self.Event Open`))

(event `Event Unlock`)

(event `Event Open Fast`
  (params (`Closewise?` :type Boolean))
  ;[1 1 1] Open & Close Door
  (set `self.Clockwise?` `Closewise?`)
  (`TimelineComponent.SetPlayRate` (`self.OpenTimeline`) 8.0)
  (`self.Event Open`))

(event `/Game/Circuit/BPI_Circuitry.SetLock`
  (params (`Unlock?` :type Boolean)))

(event `Event Open`
  ;[1 1 1] Open & Close Door
  (`GameplayStatics.PlaySoundAtLocation` (`self.OpenSlowSound`) (`self.SoundLocation`) (struct) 1.0 1.0 0.0 null null null null)
  (set `self.Open?` true)
  (bind (_direction _open) (`Timeline|OpenTimeline` :!label _label_2)
    (:`Update`
      (`self.SetDoorRotation` _open (`self.Clockwise?`)))))

(event `Event Close`
  ;[1 1 1] Open & Close Door
  (`TimelineComponent.SetPlayRate` (`self.OpenTimeline`) 1.0)
  (`GameplayStatics.PlaySoundAtLocation` (`self.CloseSound`) (`self.SoundLocation`) (struct) 1.0 1.0 0.0 null null null null)
  (set `self.Open?` false)
  (goto _label_2 :!via `Reverse`))

(event `self.ReceiveDestroyed`
  (`NiagaraFunctionLibrary.SpawnSystemAtLocation` (`self.OnDestroyedParticle`))
  (`GameplayStatics.SpawnSoundAtLocation` (`self.OnDestroyedSound`) (0.0 0.0 0.0) (struct) 1.0 1.0 0.0 null null))

(fn `InteractParent`
  (params (InteractionActor :type "Actor Object Reference"))
  (bind _returnvalue (`self.GetComponentByClass` InteractionActor "/Game/Universal/Factions/BPC_Faction.BPC_Faction_C"))
  (if (`self.Locked?`)
    ;[1 1 1] If instigator actor is a faction that can open, bypass locked door
    (`/Engine/EditorBlueprintResources/StandardMacros.IsValid` _returnvalue
      (:`Is Valid`
        (if (>= (`KismetArrayLibrary.Array_Find` (`self.FactionCanOpenLocked?`) (`/Game/Universal/Factions/BPC_Faction.Faction` _returnvalue)) 0)
          (`self.Event Open Slow` (`self.GetSwingOrientation` InteractionActor))))
      (:`Is Not Valid`))
    (elif (`self.Open?`)
      (`self.Event Close`)
      (else
        (`self.Event Open Slow` (`self.GetSwingOrientation` InteractionActor))))))

(fn `Process Lock Strength`
  (returns (`Openable?` :type Boolean))
  (return true))

(fn `SetDoorRotation`
  (params (Percent :type "Float (double-precision)") (`Clockwise?` :type Boolean))
  (bind _output_get (set `self.SwingPercent` Percent))
  (`SceneComponent.K2_SetRelativeRotation` (`self.Pivot`) (`KismetMathLibrary.MakeRotator` (* _output_get 90.0 (select `bool` `Clockwise?` :`false` 1.0 :`true` -1.0)) 90.0) false false))

(fn `UserConstructionScript`)