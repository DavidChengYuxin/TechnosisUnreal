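; BP_LeverSwitch is an environmental prop whose lever animates back and forth each time its EventAnimateButton event fires.
; A FlipFlop alternates between playing and reversing a Timeline, whose Rotation track, scaled by 180, sets the Lever component's relative roll.
; The Blueprint handles only this animation, with no overlap, tick or gameplay logic of its own.
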(event `self.Event Animate Button`
  (`/Engine/EditorBlueprintResources/StandardMacros.FlipFlop`
    (:`A`
      (bind (_direction _rotation) (`Timeline|Timeline` :!label _label)
        (:`Update`
          (`SceneComponent.K2_SetRelativeRotation` (`self.Lever`) (`KismetMathLibrary.MakeRotator` (* _rotation 180.0)) false false))))
    (:`B`
      (goto _label :!via `Reverse`))))

(fn `UserConstructionScript`
  (`parent.UserConstructionScript`))