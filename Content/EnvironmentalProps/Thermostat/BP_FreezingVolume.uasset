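; BP_FreezingVolume is a switchable volume that deals ice damage to actors inside its box.
; While on, a looping timer repeatedly applies DTBP_Ice damage to every actor overlapping the box, in place of Tick.
; The Switch event starts or clears that timer when the state changes, swapping the attached audio between on and off sounds.
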(event `self.ReceiveBeginPlay`
  (bind _returnvalue (`GameplayStatics.SpawnSoundAttached` (`self.OnSound`) (`self.DefaultSceneRoot`) "None" (0.0 0.0 0.0) (struct) "KeepRelativeOffset" false 1.0 1.0 0.0 "/Game/Audio/AttenuationPresets/ATT_Default.ATT_Default" null))
  (set `self.Audio` _returnvalue)
  (if (`self.On?`)
    (`self.Event Start Freezing`)
    (else
      (`AudioComponent.SetSound` (`self.Audio`) (`self.OffSound`)))))

(event `/Game/Circuit/BPI_Circuitry.Switch`
  (params (`On?` :type Boolean))
  (if (!= `On?` (`self.On?`))
    (bind _output_get (set `self.On?` `On?`))
    (if _output_get
      (`self.Event Start Freezing`)
      (else
        (`self.Event Stop Freezing`)))))

(event `Event Start Freezing`
  (bind _returnvalue (`KismetSystemLibrary.K2_SetTimerDelegate` (delegate `Event Freeze`) (`self.DeltaTime`) true true))
  (`AudioComponent.SetSound` (`self.Audio`) (`self.OnSound`)))

(event `Event Stop Freezing`
  (`KismetSystemLibrary.K2_ClearAndInvalidateTimerHandle` (stale `Event Start Freezing` _returnvalue))
  (`AudioComponent.SetSound` (`self.Audio`) (`self.OffSound`)))

(event `Event Freeze`
  (for _array_element (`PrimitiveComponent.GetOverlappingActors` (`self.Box`) null)
    (`GameplayStatics.ApplyDamage` _array_element 5.0 null null "/Game/ElementalDamage/Ice/DTBP_Ice.DTBP_Ice_C")))

(fn `UserConstructionScript`)