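; BP_WeakWall is a breakable wall prop that gives way to certain elemental damage.
; On BeginPlay it adds a BPC_WaterDamageable component if flagged WaterDamageable.
; AnyDamage reads the element from the damage type via BPI_Element, puncturing on Armor Piercing, or on Water when that component is present.
; Puncture swaps in the broken mesh, plays sound and particle effects, and disables mesh collision.
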(event `self.ReceiveBeginPlay`
  (if (`self.WaterDamageable?`)
    (`AddComponent|NODE_AddBPC_WaterDamageable-0`)))

(event `self.ReceiveAnyDamage`
  (params (Damage :type "Float (single-precision)") (DamageType :type "DamageType Object Reference") (InstigatedBy :type "Controller Object Reference") (DamageCauser :type "Actor Object Reference"))
  (if (`KismetSystemLibrary.DoesImplementInterface` DamageType "/Game/ElementalDamage/BPI_Element.BPI_Element_C")
    (bind _element (message `/Game/ElementalDamage/BPI_Element.GetElement` DamageType))
    (switch `/Game/ElementalDamage/Enum_Element` _element
      (:`NewEnumerator6`
        (`/Engine/EditorBlueprintResources/StandardMacros.IsValid` (`self.GetComponentByClass` "/Game/ElementalDamage/Water/BPC_WaterDamageable.BPC_WaterDamageable_C")
          (:`Is Valid`
            _)))
      (:`NewEnumerator8`
        _))
    (`self.Event Puncture`)))

(event `Event Puncture`
  (bind _mesh (`self.Mesh`))
  (bind _returnvalue (`SceneComponent.K2_GetComponentLocation` (`self.DefaultSceneRoot`)))
  (`StaticMeshComponent.SetStaticMesh` _mesh (`self.BrokenMesh`))
  (`GameplayStatics.PlaySoundAtLocation` (`self.BrokenSound`) _returnvalue (struct) 1.0 1.0 0.0 null null null null)
  (`NiagaraFunctionLibrary.SpawnSystemAttached` (`self.BrokenParticle`) null "None" _returnvalue (struct) "KeepRelativeOffset")
  (`PrimitiveComponent.SetCollisionEnabled` _mesh "NoCollision"))

(fn `UserConstructionScript`)