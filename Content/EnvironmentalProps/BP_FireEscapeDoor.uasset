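; BP_FireEscapeDoor is a fire escape door that raises an alarm when an actor interacts with it.
; Interact stores the causer as TriggerActor, runs the parent interaction, then calls TriggerAlarm.
; TriggerAlarm reports an AI noise event at that actor's location with configurable loudness and range, then forwards an alarm message with the actor to each element of an array.
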(event `/Game/Universal/Interact/BPI_Interact.Interact`
  (params (`InteractStart?` :type Boolean) (Causer :type "Actor Object Reference") (Instigator :type "Controller Object Reference"))
  (bind _output_get (set `self.TriggerActor` Causer))
  (`self.InteractParent` _output_get)
  (`/Game/EnvironmentalProps/BPI_FireAlarm.TriggerAlarm` (`self.TriggerActor`)))

(event `/Game/EnvironmentalProps/BPI_FireAlarm.TriggerAlarm`
  (params (TriggerActor :type "Actor Object Reference"))
  (bind _triggeractor (`self.TriggerActor`))
  (`AISense_Hearing.ReportNoiseEvent` (`self.K2_GetActorLocation` _triggeractor) (`self.Loudness`) _triggeractor (`self.Max Range`))
  (for _array_element _
    (message `/Game/EnvironmentalProps/BPI_FireAlarm.TriggerAlarm` _array_element (`self.TriggerActor`))))

(fn `UserConstructionScript`
  (`parent.UserConstructionScript`))