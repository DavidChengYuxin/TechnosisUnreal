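; BP_JunctionBox is an electrical prop that can be switched on and broken to act as an electrical hazard.
; Damage types reporting Kinetic, Water, Chemical, Armor Piercing or Knock Back through BPI_Element set it Broken.
; Its child electricity volume, wired up in construction, deals damage only when On and Broken, re-evaluated on Switch but not on Break.
; A temporary broken decal reflects the Broken state only at BeginPlay.
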(event `self.ReceiveBeginPlay`
  ;[1 1 1] TEMP
  (`SceneComponent.SetVisibility` (`self.TEMP Broken Decal`) (`self.Broken?`) false))

(event `/Game/Circuit/BPI_Circuitry.Switch`
  (params (`On?` :type Boolean))
  (set `self.On?` `On?`)
  (`self.Event Update State`))

(event `self.ReceiveAnyDamage`
  (params (Damage :type "Float (single-precision)") (DamageType :type "DamageType Object Reference") (InstigatedBy :type "Controller Object Reference") (DamageCauser :type "Actor Object Reference"))
  (if (`KismetSystemLibrary.DoesImplementInterface` DamageType "/Game/ElementalDamage/BPI_Element.BPI_Element_C")
    (bind _element (`/Game/Universal/BPFL_Universal.Get Element` DamageType))
    (switch `/Game/ElementalDamage/Enum_Element` _element
      (:`NewEnumerator0`
        _)
      (:`NewEnumerator6`
        _)
      (:`NewEnumerator5`
        _)
      (:`NewEnumerator8`
        _)
      (:`NewEnumerator7`
        _))
    (`self.Event Break`)))

(event `Event Update State`
  (bind _as_bp_electricity_volume (`self.As BP Electricity Volume`))
  (bind _output_get (set `/Game/ElementalDamage/BP_ElementalDamageVolume.Active?` (and (`self.On?`) (`self.Broken?`)) _as_bp_electricity_volume))
  (if _output_get
    (`/Game/ElementalDamage/BP_ElementalDamageVolume.Event Start Damage` _as_bp_electricity_volume)
    (else
      (`/Game/ElementalDamage/BP_ElementalDamageVolume.Event Stop Damage` _as_bp_electricity_volume))))

(event `Event Break`
  (set `self.Broken?` true))

(fn `UserConstructionScript`
  (bind _asbp_electricity_volume (cast `/Game/ElementalDamage/Electricity/BP_ElectricityVolume` (`ChildActorComponent.ChildActor` (`self.ElectricityVolume`))))
  (bind _output_get (set `self.As BP Electricity Volume` _asbp_electricity_volume))
  (set `/Game/ElementalDamage/BP_ElementalDamageVolume.Damage Causer` self _output_get)
  (`self.Event Update State`))