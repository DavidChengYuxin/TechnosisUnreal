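; BP_CircuitManager is an electrical prop actor that relays an on/off switch signal to a group of linked actors.
; Its Switch event stores the On state and forwards it through SwitchMessage to every entry in the Circuitry array.
; On BeginPlay it removes Circuit Manager instances and their subclasses from that array to avoid infinite loops, though it does so while iterating the same array.
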(event `self.ReceiveBeginPlay`
  ;[1 1 1] Remove instances of Circuit Manager (avoids infinite loops)
  (for _array_element (`self.Circuitry`)
    (if (`KismetMathLibrary.ClassIsChildOf` (`GameplayStatics.GetObjectClass` _array_element) "BP_CircuitManager_C")
      (`KismetArrayLibrary.Array_RemoveItem` (`self.Circuitry`) _array_element))))

(event `/Game/Circuit/BPI_Circuitry.Switch`
  (params (`On?` :type Boolean))
  (bind _output_get (set `self.On?` `On?`))
  (for _array_element (`self.Circuitry`)
    (message `/Game/Circuit/BPI_Circuitry.Switch` _array_element _output_get)))

(fn `UserConstructionScript`)