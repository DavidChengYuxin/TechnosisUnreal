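; Fire sprinkler prop that reacts to elemental damage taken by actors in the area beneath it.
; Its construction script traces downward to size the detection box to the floor and cache a puddle transform.
; Actors in the box get their damage events bound, and a matching BPI_Element damage type triggers the sprinkler.
; First activation spawns the effect system and a BP_WaterPuddle, while water damage logic is left disconnected.
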(event `self.ReceiveBeginPlay`
  ;[1 1 1] Allows actors in radius at spawn to be affected
  (for _array_element (`PrimitiveComponent.GetOverlappingActors` (`self.Box`) null)
    (add `self.OnTakeAnyDamage` _array_element (delegate `Event Actors Recieved Damage?`))
    (`KismetArrayLibrary.Array_Add` (`self.Overlapping Actors`) _array_element)))

(event `self.Box.OnComponentBeginOverlap`
  (params (OverlappedComponent :type "PrimitiveComponent Object Reference") (OtherActor :type "Actor Object Reference") (OtherComp :type "PrimitiveComponent Object Reference") (OtherBodyIndex :type Integer) (bFromSweep :type Boolean) (SweepResult :type "HitResult Structure (by ref)"))
  (add `self.OnTakeAnyDamage` OtherActor (delegate `Event Actors Recieved Damage?`))
  (`KismetArrayLibrary.Array_Add` (`self.Overlapping Actors`) OtherActor))

(event `Event Actors Recieved Damage?` :!signature `self.OnTakeAnyDamage`
  (params (DamagedActor :type "Actor Object Reference") (Damage :type "Float (single-precision)") (DamageType :type "DamageType Object Reference") (InstigatedBy :type "Controller Object Reference") (DamageCauser :type "Actor Object Reference"))
  (if (`KismetSystemLibrary.DoesImplementInterface` DamageType "/Game/ElementalDamage/BPI_Element.BPI_Element_C")
    (bind _element (message `/Game/ElementalDamage/BPI_Element.GetElement` DamageType))
    (if (`|EnumEquality` _element "NewEnumerator1")
      (`self.Event Activate Sprinkler`))))

(event `self.Box.OnComponentEndOverlap`
  (params (OverlappedComponent :type "PrimitiveComponent Object Reference") (OtherActor :type "Actor Object Reference") (OtherComp :type "PrimitiveComponent Object Reference") (OtherBodyIndex :type Integer))
  (remove `self.OnTakeAnyDamage` OtherActor (delegate `Event Actors Recieved Damage?`))
  (`KismetArrayLibrary.Array_RemoveItem` (`self.Overlapping Actors`) OtherActor))

(event `Event Activate Sprinkler`
  (bind (_returnvalue_location _returnvalue_rotation) (`KismetMathLibrary.BreakTransform` (`SceneComponent.K2_GetComponentToWorld` (`self.Mesh`))))
  (if (`self.SprinklerActive?`)
    (`TimelineComponent.PlayFromStart` (`self.Timeline`))
    (else
      (set `self.SprinklerActive?` true)
      (`NiagaraFunctionLibrary.SpawnSystemAtLocation` (`self.System Template`) _returnvalue_location _returnvalue_rotation)
      (bind _returnvalue (`|SpawnActorFromClass` "/Game/ElementalDamage/Water/BP_WaterPuddle.BP_WaterPuddle_C" (`self.WaterPuddleSpawnTransform`) "Undefined" "MultiplyWithRoot" null null)))))

(event `Event Stop Sprinkler`
  (set `self.SprinklerActive?` false))

(fn `UserConstructionScript`
  (bind _box (`self.Box`))
  (bind _returnvalue (`SceneComponent.K2_GetComponentLocation` (`self.Mesh`)))
  (bind (_outhit _returnvalue_2) (`KismetSystemLibrary.LineTraceSingle` _returnvalue (+ _returnvalue (* (`KismetMathLibrary.Vector_Up`) -3000.0)) "TraceTypeQuery1"))
  (if _returnvalue_2
    (bind (_bblockinghit _binitialoverlap _time _distance _location _impactpoint _normal) (`GameplayStatics.BreakHitResult` _outhit))
    (set `self.WaterPuddleSpawnTransform` (`KismetMathLibrary.MakeTransform` _impactpoint (`KismetMathLibrary.MakeRotFromZ` _normal) (1.0 2.5 2.5)))
    (bind _returnvalue_3 (select `bool` _returnvalue_2 :`false` 1000.0 :`true` _distance))
    (`SceneComponent.K2_SetRelativeLocation` _box (`KismetMathLibrary.MakeVector` 0.0 0.0 (* _returnvalue_3 -0.5)) false false)
    (`BoxComponent.SetBoxExtent` _box (`KismetMathLibrary.MakeVector` 500.0 500.0 (* _returnvalue_3 0.5)) true)))