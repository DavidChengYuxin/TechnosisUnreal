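; Vent door cover prop that can be opened, closed or removed when opened fast, as when kicked.
; A slow open plays a sound at the pivot and runs a timeline whose Out and Up tracks move the door's relative X and Z location.
; Closing plays its own sound and reverses that timeline, while a fast open simply destroys the actor with no sound or animation.
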(event `self.Event Open Fast`
  (params (`Closewise?` :type Boolean))
  ;[0.315 0.315 0.315] Destory actor on open fast (i.e. kicked)
  (`self.K2_DestroyActor`))

(event `self.Event Open`
  (`GameplayStatics.PlaySoundAtLocation` (`self.OpenSlowSound`) (`SceneComponent.K2_GetComponentLocation` (`self.Pivot`)) (struct) 1.0 1.0 0.0 null null null null)
  (set `self.Open?` true)
  (bind (_direction _out _up) (`Timeline|Timeline` :!label _label)
    (:`Update`
      (`SceneComponent.K2_SetRelativeLocation` (`self.Door`) (`KismetMathLibrary.MakeVector` _out 0.0 _up) false false))))

(event `self.Event Close`
  (`GameplayStatics.PlaySoundAtLocation` (`self.CloseSound`) (`SceneComponent.K2_GetComponentLocation` (`self.Pivot`)) (struct) 1.0 1.0 0.0 null null null null)
  (set `self.Open?` false)
  (goto _label :!via `Reverse`))

(fn `UserConstructionScript`
  (`parent.UserConstructionScript`))