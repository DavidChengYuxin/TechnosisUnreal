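; Fire alarm prop that, once triggered, repeatedly plays an alarm sound and reports AI noise until reset.
; TriggerAlarm stores the triggering actor, sounds immediately, then starts a looping timer that ResetAlarm clears.
; Each pulse plays audio at the alarm but reports noise at the trigger actor's location, with that actor as instigator.
; Loudness scales with alarm-to-actor distance over MaxRange, so it grows louder as the actor gets farther away.
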(event `Event Alarm Sound`
  (bind _returnvalue (`self.K2_GetActorLocation`))
  (bind _max_range (`self.Max Range`))
  (bind _trigger_actor (`self.Trigger Actor`))
  (bind _returnvalue_2 (`self.K2_GetActorLocation` _trigger_actor))
  (`GameplayStatics.PlaySoundAtLocation` (`self.FireAlarm`) _returnvalue (struct) 1.0 1.0 0.0 null null null null)
  (`AISense_Hearing.ReportNoiseEvent` _returnvalue_2 (* (`self.MaxLoudness`) (/ (`KismetMathLibrary.VSize` (- _returnvalue _returnvalue_2)) _max_range)) _trigger_actor _max_range))

(event `/Game/EnvironmentalProps/FireSystem/BPI_FireAlarm.TriggerAlarm`
  (params (TriggerActor :type "Actor Object Reference"))
  (set `self.Trigger Actor` TriggerActor)
  (`self.Event Alarm Sound`)
  (bind _returnvalue (`KismetSystemLibrary.K2_SetTimerDelegate` (delegate `Event Alarm Sound`) (`self.DelaySeconds`) true true))
  (set `self.AlarmTimer` _returnvalue))

(event `/Game/EnvironmentalProps/FireSystem/BPI_FireAlarm.ResetAlarm`
  (`KismetSystemLibrary.K2_ClearAndInvalidateTimerHandle` (`self.AlarmTimer`)))

(fn `UserConstructionScript`)