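; Fire escape door, a child Blueprint that raises the fire alarm system when opened.
; Damage and interaction record the responsible actor as TriggerActor before passing to the parent logic.
; On opening, it passes that actor to FireAlarmSystem's manager message and plays a timeline sliding two push bars.
; TriggerAlarm reports a noise event at the triggering actor's location, with configurable loudness and range.
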(event `self.ReceiveAnyDamage`
  (params (Damage :type "Float (single-precision)") (DamageType :type "DamageType Object Reference") (InstigatedBy :type "Controller Object Reference") (DamageCauser :type "Actor Object Reference"))
  (bind _output_get (set `self.TriggerActor` DamageCauser))
  (`parent.ReceiveAnyDamage` Damage DamageType InstigatedBy _output_get))

(event `/Game/Universal/Interact/BPI_Interact.Interact`
  (params (`InteractStart?` :type Boolean) (Causer :type "Actor Object Reference") (Instigator :type "Controller Object Reference"))
  (bind _output_get (set `self.TriggerActor` Causer))
  (`parent.Interact` `InteractStart?` _output_get Instigator))

(event `self.Event Open`
  (`parent.Event Open`)
  (message `/Game/EnvironmentalProps/FireSystem/BPI_FireAlarm.TriggerCallManager` (`self.FireAlarmSystem`) (`self.TriggerActor`))
  (bind (_direction _location) (`Timeline|Timeline` :!via `PlayFromStart`)
    (:`Update`
      (`SceneComponent.K2_SetRelativeLocation` (`self.PushBar1`) (`KismetMathLibrary.MakeVector` (* _location 50.0) 0.0 -10.0) false false)
      (`SceneComponent.K2_SetRelativeLocation` (`self.PushBar2`) (`KismetMathLibrary.MakeVector` (* _location -50.0) 0.0 -10.0) false false))))

(event `/Game/EnvironmentalProps/FireSystem/BPI_FireAlarm.TriggerAlarm`
  (params (TriggerActor :type "Actor Object Reference"))
  (`AISense_Hearing.ReportNoiseEvent` (`self.K2_GetActorLocation` TriggerActor) (`self.Loudness`) TriggerActor (`self.Max Range`)))

(fn `UserConstructionScript`
  (`parent.UserConstructionScript`))