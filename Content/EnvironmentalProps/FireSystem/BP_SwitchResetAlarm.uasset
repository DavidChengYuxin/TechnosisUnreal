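; BP_SwitchResetAlarm is an interactable switch in the fire system that resets the fire alarm.
; It extends its parent's Interact event, running the parent logic first and then, only when an interaction starts, calling ResetCallManagerMessage on its FireAlarmSystem reference.
; The construction script only calls the parent, and the BeginPlay, overlap and Tick events are disabled.
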(event `/Game/Universal/Interact/BPI_Interact.Interact`
  (params (`InteractStart?` :type Boolean) (Causer :type "Actor Object Reference") (Instigator :type "Controller Object Reference"))
  (`parent.Interact` `InteractStart?` Causer Instigator)
  (if `InteractStart?`
    (message `/Game/EnvironmentalProps/FireSystem/BPI_FireAlarm.ResetCallManager` (`self.FireAlarmSystem`))))

(fn `UserConstructionScript`
  (`parent.UserConstructionScript`))