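; Fire sprinkler that triggers when an overlapping actor takes matching elemental damage or enters burning.
; At BeginPlay, a downward trace sizes its detection box to the floor and sets the puddle spawn point.
; Activation spawns particles and a puddle, applies water damage to occupants and raises the sound volume.
; Later entrants also take water damage while it runs, until a timer, reset by each trigger, stops it.
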(event `self.ReceiveBeginPlay`
  (`self.SetUpVolume`)
  ;[1 1 1] Allows actors in radius at spawn to be affected
  (for _array_element (`PrimitiveComponent.GetOverlappingActors` (`self.Box`) null)
    (add `self.OnTakeAnyDamage` _array_element (delegate `Event Actors Recieved Damage?`))
    (`KismetArrayLibrary.Array_Add` (`self.Overlapping Actors`) _array_element)))

(event `self.Box.OnComponentBeginOverlap`
  (params (OverlappedComponent :type "PrimitiveComponent Object Reference") (OtherActor :type "Actor Object Reference") (OtherComp :type "PrimitiveComponent Object Reference") (OtherBodyIndex :type Integer) (bFromSweep :type Boolean) (SweepResult :type "HitResult Structure (by ref)"))
  (bind _returnvalue (`self.GetComponentByClass` OtherActor "/Game/ElementalDamage/Fire/BPC_Flammable.BPC_Flammable_C"))
  (add `self.OnTakeAnyDamage` OtherActor (delegate `Event Actors Recieved Damage?`))
  (`KismetArrayLibrary.Array_Add` (`self.Overlapping Actors`) OtherActor)
  (if (`self.SprinklerActive?`)
    (`GameplayStatics.ApplyDamage` OtherActor (`self.Sprinkler Water Damage`) (`self.Instigated By`) (`self.Damage Causer`) "/Game/ElementalDamage/Water/DTBP_Water.DTBP_Water_C" :!label _label)
    (else
      (`/Engine/EditorBlueprintResources/StandardMacros.IsValid` _returnvalue
        (:`Is Valid`
          (if (`/Game/ElementalDamage/Fire/BPC_Flammable.Burning?` _returnvalue)
            (`self.Event Activate Sprinkler`)
            (goto _label)))
        (:`Is Not Valid`)))))

(event `Event Actors Recieved Damage?` :!signature `self.OnTakeAnyDamage`
  (params (DamagedActor :type "Actor Object Reference") (Damage :type "Float (single-precision)") (DamageType :type "DamageType Object Reference") (InstigatedBy :type "Controller Object Reference") (DamageCauser :type "Actor Object Reference"))
  (if (`KismetSystemLibrary.DoesImplementInterface` DamageType "/Game/ElementalDamage/BPI_Element.BPI_Element_C")
    (bind _element (message `/Game/ElementalDamage/BPI_Element.GetElement` DamageType))
    (if (`|EnumEquality` _element "NewEnumerator1")
      (`self.Event Activate Sprinkler`)
      (set `self.Instigated By` InstigatedBy)
      (set `self.Damage Causer` DamageCauser))))

(event `self.Box.OnComponentEndOverlap`
  (params (OverlappedComponent :type "PrimitiveComponent Object Reference") (OtherActor :type "Actor Object Reference") (OtherComp :type "PrimitiveComponent Object Reference") (OtherBodyIndex :type Integer))
  (remove `self.OnTakeAnyDamage` OtherActor (delegate `Event Actors Recieved Damage?`))
  (`KismetArrayLibrary.Array_RemoveItem` (`self.Overlapping Actors`) OtherActor))

(event `Event Activate Sprinkler`
  (bind (_returnvalue_location _returnvalue_rotation) (`KismetMathLibrary.BreakTransform` (`SceneComponent.K2_GetComponentToWorld` (`self.Mesh`))))
  (`KismetSystemLibrary.K2_SetTimerDelegate` (delegate `Event Stop Sprinkler`) (`self.SprinklerRunTime`))
  (if (not (`self.SprinklerActive?`))
    (`|ExecutionSequence`
      (:`then_0`
        (set `self.SprinklerActive?` true))
      (:`then_1`
        (`NiagaraFunctionLibrary.SpawnSystemAtLocation` (`self.System Template`) _returnvalue_location _returnvalue_rotation))
      (:`then_2`
        (`|SpawnActorFromClass` "/Game/ElementalDamage/Water/BP_WaterPuddle.BP_WaterPuddle_C" (`self.WaterPuddleSpawnTransform`) "AlwaysSpawn" "MultiplyWithRoot" null null))
      (:`then_3`
        (for _array_element (`self.Overlapping Actors`)
          (`GameplayStatics.ApplyDamage` _array_element (`self.Sprinkler Water Damage`) (`self.Instigated By`) (`self.Damage Causer`) "/Game/ElementalDamage/Water/DTBP_Water.DTBP_Water_C")))
      (:`then_4`
        (`AudioComponent.SetVolumeMultiplier` (`self.Sound`) 1.0)))))

(event `Event Stop Sprinkler`
  (set `self.SprinklerActive?` false)
  (`AudioComponent.SetVolumeMultiplier` (`self.Sound`) 0.0))

(fn `SetUpVolume`
  (bind _box (`self.Box`))
  (bind _returnvalue (`SceneComponent.K2_GetComponentLocation` (`self.Mesh`)))
  (bind _outactors (`GameplayStatics.GetAllActorsOfClass` "/Game/Props/BP_Grabbable_Parent.BP_Grabbable_Parent_C"))
  (bind (_outhit _returnvalue_2) (`KismetSystemLibrary.LineTraceSingle` _returnvalue (+ _returnvalue (* (`KismetMathLibrary.Vector_Up`) -3000.0)) "TraceTypeQuery1" false _outactors))
  (if _returnvalue_2
    (bind (_bblockinghit _binitialoverlap _time _distance _location _impactpoint _normal) (`GameplayStatics.BreakHitResult` _outhit))
    (set `self.WaterPuddleSpawnTransform` (`KismetMathLibrary.MakeTransform` _impactpoint (`KismetMathLibrary.MakeRotFromZ` _normal) (1.0 2.5 2.5)))
    (bind _returnvalue_3 (select `bool` _returnvalue_2 :`false` 1000.0 :`true` _distance))
    (`SceneComponent.K2_SetRelativeLocation` _box (`KismetMathLibrary.MakeVector` 0.0 0.0 (* _returnvalue_3 -0.5)) false false)
    (`BoxComponent.SetBoxExtent` _box (`KismetMathLibrary.MakeVector` 500.0 500.0 (* _returnvalue_3 0.5)) true)))

(fn `UserConstructionScript`)