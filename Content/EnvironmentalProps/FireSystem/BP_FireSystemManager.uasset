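; BP_FireSystemManager is a manager actor that relays alarm triggers and resets to the actors in a fire system.
; TriggerCallManager stores the triggering actor, passes it to every entry in ActorsInSystem through TriggerAlarmMessage, then sets an auto-reset timer using TimeAutoReset.
; ResetCallManager, fired by that timer or called directly, sends ResetAlarmMessage to every actor and clears the timer.
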(event `/Game/EnvironmentalProps/FireSystem/BPI_FireAlarm.TriggerCallManager`
  (params (TriggerActor :type "Actor Object Reference"))
  (set `self.Trigger Actor` TriggerActor)
  (for _array_element (`self.ActorsInSystem`)
    (message `/Game/EnvironmentalProps/FireSystem/BPI_FireAlarm.TriggerAlarm` _array_element (`self.Trigger Actor`)))
  (bind _returnvalue (`KismetSystemLibrary.K2_SetTimerDelegate` (delegate `/Game/EnvironmentalProps/FireSystem/BPI_FireAlarm.ResetCallManager`) (`self.TimeAutoReset`) false true))
  (set `self.AutoResetTimer` _returnvalue))

(event `/Game/EnvironmentalProps/FireSystem/BPI_FireAlarm.ResetCallManager`
  (for _array_element (`self.ActorsInSystem`)
    (message `/Game/EnvironmentalProps/FireSystem/BPI_FireAlarm.ResetAlarm` _array_element))
  (`KismetSystemLibrary.K2_ClearAndInvalidateTimerHandle` (`self.AutoResetTimer`)))

(fn `UserConstructionScript`)