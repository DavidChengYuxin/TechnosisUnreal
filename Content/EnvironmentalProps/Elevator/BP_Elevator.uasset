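; BP_Elevator is an elevator prop meant to travel between ElevatorStop locations, though its movement is not wired up.
; CallElevator stores the requested stop and its location as the next target when it differs from CurrentStop, and Switch sets the On flag.
; Disconnected logic would spring-interpolate the root toward that target and update CurrentStop, but nothing runs it, so the elevator never moves itself.
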(event `/Game/Circuit/BPI_Circuitry.Switch`
  (params (`On?` :type Boolean))
  (set `self.On?` `On?`))

(event `/Game/Circuit/BPI_Circuitry.CallElevator`
  (params (ElevatorStop :type "/Game/EnvironmentalProps/Elevator/BP_ElevatorStop Object Reference"))
  (if (!= ElevatorStop (`self.CurrentStop`))
    (bind _output_get (set `self.NextStop` ElevatorStop))
    (set `self.NextLocation` (`self.K2_GetActorLocation` _output_get))))

(fn `UserConstructionScript`)