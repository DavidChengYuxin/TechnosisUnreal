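; BP_ElevatorStop is an elevator stop that opens or closes the doors assigned to it.
; Two identical custom events, CallElevatorDoor and CallElevatorDoor_1, take an Open flag and loop over the ElevatorDoor array, calling EventOpen or EventClose on each entry.
; It has no active BeginPlay, overlap, Tick or construction logic, so it acts only when one of these events is called.
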(event `CallElevatorDoor_1`
  (params (`Open?` :type Boolean))
  (for _array_element (`self.ElevatorDoor`)
    (if `Open?`
      (`/Game/EnvironmentalProps/BP_Door_Parent.Event Open` _array_element)
      (else
        (`/Game/EnvironmentalProps/BP_Door_Parent.Event Close` _array_element)))))

(event `Event Call Elevator Door`
  (params (`Open?` :type Boolean))
  (for _array_element (`self.ElevatorDoor`)
    (if `Open?`
      (`/Game/EnvironmentalProps/BP_Door_Parent.Event Open` _array_element)
      (else
        (`/Game/EnvironmentalProps/BP_Door_Parent.Event Close` _array_element)))))

(fn `UserConstructionScript`)