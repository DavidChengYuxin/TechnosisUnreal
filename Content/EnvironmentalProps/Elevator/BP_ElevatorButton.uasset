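; BP_ElevatorButton is a button that calls its referenced elevator to a set stop when interacted with or pressed.
; Interact and PressButton share one sequence that sends the call, plays a 2D sound and runs a timeline moving the mesh along relative Z.
; A Switch event stores an On flag, which the press logic does not check.
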(event `self.Interact`
  (params (`InteractStart?` :type Boolean) (Causer :type "Actor Object Reference") (Instigator :type "Controller Object Reference"))
  (`|ExecutionSequence` :!label _label
    (:`then_0`
      (`/Game/EnvironmentalProps/Elevator/BP_Elevator.Event Call Elevator` (`self.Elevator`) (`self.ElevatorStop`)))
    (:`then_1`
      (`GameplayStatics.PlaySound2D` (`self.Sound`) 1.0 1.0 0.0 null null))
    (:`then_2`
      (bind (_direction _height) (`Timeline|Timeline` :!via `PlayFromStart`)
        (:`Update`
          (`SceneComponent.K2_SetRelativeLocation` (`self.Mesh`) (`KismetMathLibrary.MakeVector` 0.0 0.0 (* _height 5.0)) false false))))))

(event `Event Press Button`
  (goto _label))

(event `/Game/Circuit/BPI_Circuitry.Switch`
  (params (`On?` :type Boolean))
  (set `self.On?` `On?`))

(fn `UserConstructionScript`)