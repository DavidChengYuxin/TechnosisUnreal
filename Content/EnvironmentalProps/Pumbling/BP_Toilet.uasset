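; Interactable toilet prop that flushes when used, dealing water damage to actors around it.
; Construction sets the interaction type on BPCInteractable, and the Interact event feeds Flush, which acts only on interaction start while ready.
; A flush spawns an attached particle system, plays a sound, applies water damage to everything overlapping the Box, then re-arms after a short delay.
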(event `/Game/Universal/Interact/BPI_Interact.Interact`
  (params (`InteractStart?` :type Boolean) (Causer :type "Actor Object Reference") (Instigator :type "Controller Object Reference"))
  (if (and `InteractStart?` (`self.Ready?`))
    (`|ExecutionSequence`
      (:`then_0`
        (set `self.Ready?` false))
      (:`then_1`
        (`self.PlayAnimation`))
      (:`then_2`
        (for _array_element (`PrimitiveComponent.GetOverlappingActors` (`self.Box`) null)
          (`GameplayStatics.ApplyDamage` _array_element 15.0 Instigator Causer "/Game/ElementalDamage/Water/DTBP_Water.DTBP_Water_C")))
      (:`then_3`
        (`KismetSystemLibrary.Delay` 3.0)
        (set `self.Ready?` true)))))

(event `PlayAnimation`
  (`NiagaraFunctionLibrary.SpawnSystemAttached` null null "None" (0.0 0.0 0.0) (struct) "KeepRelativeOffset")
  (`GameplayStatics.PlaySoundAtLocation` (`self.UseSound`) (`SceneComponent.K2_GetComponentLocation` (`self.Box`)) (struct) 1.0 1.0 0.0 null null null null))

(fn `UserConstructionScript`
  (set `/Game/Universal/Interact/BPC_Interactable.InteractionType` "NewEnumerator1" (`self.BPC_Interactable`)))