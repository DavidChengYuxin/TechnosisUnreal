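; BPC_Health is an actor component that tracks health, alive and conscious state for its owner.
; Processed damage reduces Health and triggers Death at zero, while non-lethal elemental damage, identified through BPI_Element, triggers Unconscious.
; Both events call SetConscious, which for AI-controlled owners updates the Blackboard, toggles perception senses and switches the BPC_Interactable type, adding one if missing, to make NPCs grabbable.
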(event `Event Recieve Processed Damage`
  (params (Damage :type "Float (double-precision)"))
  (bind _output_get (set `self.Health` (- (`self.Health`) Damage)))
  (if (<= _output_get 0.0)
    (`self.Event Death`)))

(event `Event Death`
  (`self.SetConscious` false)
  (set `self.Alive?` false))

(event `Event Unconscious`
  (`self.SetConscious` false))

(fn `ProcessElementalDamage`
  (params (Damage :type "Float (double-precision)") (DamageType :type "DamageType Object Reference") (InstigatedBy :type "Controller Object Reference") (DamageCauser :type "Actor Object Reference"))
  (locals (DamageElement :type "/Game/ElementalDamage/Enum_Element Enum" :default "NewEnumerator0"))
  (if (`KismetSystemLibrary.DoesImplementInterface` DamageType "/Game/ElementalDamage/BPI_Element.BPI_Element_C")
    (bind _element (message `/Game/ElementalDamage/BPI_Element.GetElement` DamageType))
    (bind _output_get (set `local.DamageElement` _element))
    (switch `/Game/ElementalDamage/Enum_Element` _output_get
      (:`NewEnumerator4`
        (`self.Event Unconscious`)))))

(fn `SetConscious`
  (params (`Conscious?` :type Boolean))
  (locals (AllSenseClasses :type "Array of AISense Class Reference") (`As BPC Interactable` :type "/Game/UniversalActorComponents/Interact/BPC_Interactable Object Reference"))
  (bind _returnvalue (`self.GetOwner`))
  (bind _returnvalue_2 (`Actor.GetComponentByClass` _returnvalue "/Game/UniversalActorComponents/Interact/BPC_Interactable.BPC_Interactable_C"))
  (bind _returnvalue_3 (`AIBlueprintHelperLibrary.GetAIController` (`self.GetOwner`)))
  (bind _output_get (set `self.Conscious?` `Conscious?`))
  ;[1 1 1] Updates AI Blackboard IFF parent is an NPC
  (`/Engine/EditorBlueprintResources/StandardMacros.IsValid` _returnvalue_3
    (:`Is Valid`
      (`BlackboardComponent.SetValueAsBool` (`AIController.Blackboard` _returnvalue_3) "Conscious?" _output_get)
      (for _array_element (`local.AllSenseClasses`)
        (`AIPerceptionComponent.SetSenseEnabled` (`AIController.GetAIPerceptionComponent` _returnvalue_3) _array_element (`self.Conscious?`))
        ;;[1 1 1] Set NPC as grabbable
        (`/Engine/EditorBlueprintResources/StandardMacros.IsValid` _returnvalue_2
          (:`Is Valid`
            (set `local.As BPC Interactable` _returnvalue_2))
          (:`Is Not Valid`
            (bind _returnvalue_4 (`|AddComponentByClass` _returnvalue "/Game/UniversalActorComponents/Interact/BPC_Interactable.BPC_Interactable_C"))
            (set `local.As BPC Interactable` _returnvalue_4)))
        (set `/Game/UniversalActorComponents/Interact/BPC_Interactable.InteractionType` (select `bool` (`self.Conscious?`) :`false` "NewEnumerator2" :`true` "NewEnumerator3" :!type "/Game/UniversalActorComponents/Interact/Enum_Interaction Enum") (`local.As BPC Interactable`))))))