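; BP_HealthPack is an interactable health pack item that adds to the interacting actor's health pack count.
; It overrides Interact, calls the parent implementation, then on interaction start increments HealthPack on the Causer's BPC_Inventory component if one exists.
; It applies no healing itself, and any other behavior, such as removing the pickup, is left to the parent class.
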(event `/Game/Universal/Interact/BPI_Interact.Interact`
  (params (`InteractStart?` :type Boolean) (Causer :type "Actor Object Reference") (Instigator :type "Controller Object Reference"))
  (bind _returnvalue (`self.GetComponentByClass` Causer "/Game/Items/BPC_Inventory.BPC_Inventory_C"))
  (`parent.Interact` `InteractStart?` Causer Instigator)
  (if (and `InteractStart?` (`KismetSystemLibrary.IsValid` _returnvalue))
    (`/Engine/EditorBlueprintResources/StandardMacros.IncrementInt` (`/Game/Items/BPC_Inventory.HealthPack` _returnvalue))))

(fn `UserConstructionScript`
  (`parent.UserConstructionScript`))