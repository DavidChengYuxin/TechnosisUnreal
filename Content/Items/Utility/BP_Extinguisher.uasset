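; Handheld fire extinguisher item that sprays water damage while triggered and can burst in a steam explosion.
; Trigger runs a per-frame looping timer that applies radial water damage at the nozzle, plays sound, attaches steam once per press and drains Usage until despawn.
; Certain damage types, or knockback and impacts above an impulse threshold, detonate it with falloff water damage, sound and particles.
; Despawning differs when the item has a parent actor.
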(event `/Game/Items/BPI_Item.Trigger`
  (params (`Start?` :type Boolean))
  (if `Start?`
    (bind _returnvalue (`KismetSystemLibrary.K2_SetTimerDelegate` (delegate `Event Spray`) (`GameplayStatics.GetWorldDeltaSeconds`) true true))
    (else
      (`KismetSystemLibrary.K2_ClearAndInvalidateTimerHandle` _returnvalue)
      (`ActorComponent.K2_DestroyComponent` (stale `Event Spray` _returnvalue))
      (goto _label_2 :!via `Reset`))))

(event `self.ReceiveAnyDamage`
  (params (Damage :type "Float (single-precision)") (DamageType :type "DamageType Object Reference") (InstigatedBy :type "Controller Object Reference") (DamageCauser :type "Actor Object Reference"))
  (`/Game/Universal/BPML_Universal.SwitchOnElementalDamage` DamageType
    (:`Kinetic`
      (`self.Event Explode` :!label _label))
    (:`Ice`
      (goto _label))
    (:`Chemical`
      (goto _label))
    (:`ArmorPiercing`
      (goto _label))
    (:`KnockBack`
      (if (>= Damage (`self.MinImpulseToExplode`))
        (`self.Event Explode`)))))

(event `Event Spray`
  (`|ExecutionSequence`
    (:`then_0`
      (`GameplayStatics.ApplyRadialDamage` :`BaseDamage` (* (`self.WaterDPS`) (`GameplayStatics.GetWorldDeltaSeconds`)) :`Origin` (`SceneComponent.K2_GetComponentLocation` (`self.Nozzle`)) :`DamageRadius` 500.0 :`DamageTypeClass` "/Game/ElementalDamage/Water/DTBP_Water.DTBP_Water_C" :`DamageCauser` (`self.ParentActor`) :`InstigatedByController` null :`bDoFullDamage` true :`DamagePreventionChannel` "ECC_Camera"))
    (:`then_1`
      (`/Engine/EditorBlueprintResources/StandardMacros.DoOnce` false :!label _label_2
        (:`Completed`
          (bind _returnvalue (`NiagaraFunctionLibrary.SpawnSystemAttached` "/Game/Effects/InfinityBladeEffects/Effects/FX_Cines/cinema03/P_CIN_03_WaterDipSteam_Converted.P_CIN_03_WaterDipSteam_Converted" (`self.Nozzle`) "None" (0.0 0.0 0.0) (struct) "KeepRelativeOffset")))))
    (:`then_2`
      (`GameplayStatics.PlaySound2D` "/Game/SoundEffects/FreeSound/kwahmah/246329__kwahmah_02__aerosol_spray.246329__kwahmah_02__aerosol_spray" 1.0 1.0 0.0 null null))
    (:`then_3`
      (bind _output_get (set `self.Usage` (- (`self.Usage`) (`GameplayStatics.GetWorldDeltaSeconds`))))
      (if (<= _output_get 0.0)
        (`self.DespawnWhileEquipped`)))))

(event `self.ReceiveHit`
  (params (MyComp :type "PrimitiveComponent Object Reference") (Other :type "Actor Object Reference") (OtherComp :type "PrimitiveComponent Object Reference") (bSelfMoved :type Boolean) (HitLocation :type "Vector Structure") (HitNormal :type "Vector Structure") (NormalImpulse :type "Vector Structure") (Hit :type "HitResult Structure (by ref)"))
  (`parent.ReceiveHit` MyComp Other OtherComp bSelfMoved HitLocation HitNormal NormalImpulse Hit)
  (if (>= (`KismetMathLibrary.VSize` NormalImpulse) (`self.MinImpulseToExplode`))
    (`self.Event Explode`)))

(event `Event Explode`
  (bind (_returnvalue_location _returnvalue_rotation) (`KismetMathLibrary.BreakTransform` (`SceneComponent.K2_GetComponentToWorld` (`self.DefaultSceneRoot`))))
  (`|ExecutionSequence`
    (:`then_0`
      (`GameplayStatics.ApplyRadialDamageWithFalloff` :`BaseDamage` 50.0 :`Origin` (`SceneComponent.K2_GetComponentLocation` (`self.DefaultSceneRoot`)) :`DamageInnerRadius` 300.0 :`DamageOuterRadius` 1000.0 :`DamageFalloff` 1.0 :`DamageTypeClass` "/Game/ElementalDamage/Water/DTBP_Water.DTBP_Water_C" :`DamageCauser` null :`InstigatedByController` null))
    (:`then_1`
      (`GameplayStatics.PlaySound2D` "/Game/Audio/Sounds/Explosions/Explosions_Grenade_Noise-Exterior-Distant_03.Explosions_Grenade_Noise-Exterior-Distant_03" 1.0 1.0 0.0 null null))
    (:`then_2`
      (`NiagaraFunctionLibrary.SpawnSystemAtLocation` "/Game/Effects/InfinityBladeEffects/Effects/FX_Monsters/FX_Monster_Bear/NS_SteamExplosion.NS_SteamExplosion" _returnvalue_location _returnvalue_rotation))
    (:`then_3`
      (`/Engine/EditorBlueprintResources/StandardMacros.IsValid` (`self.ParentActor`)
        (:`Is Valid`
          (`self.DespawnWhileEquipped`))
        (:`Is Not Valid`
          (`self.K2_DestroyActor`))))))

(fn `UserConstructionScript`
  (`parent.UserConstructionScript`))