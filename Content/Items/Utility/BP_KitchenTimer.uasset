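; Throwable kitchen timer item that ticks down and rings, reporting an AI noise event when it goes off.
; Trigger press or Alt adds time and starts a looping countdown timer that rotates the dial and plays tick sounds.
; Trigger release launches it from its parent, passing remaining time and countdown state to the released timer.
; Impacts apply minor kinetic damage to whatever it hits.
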(event `self.ReceiveAnyDamage`
  (params (Damage :type "Float (single-precision)") (DamageType :type "DamageType Object Reference") (InstigatedBy :type "Controller Object Reference") (DamageCauser :type "Actor Object Reference"))
  (switch `/Game/ElementalDamage/Enum_Element` (`/Game/Universal/BPFL_Universal.Get Element` DamageType)))

(event `self.Trigger`
  (params (`Start?` :type Boolean))
  (if `Start?`
    (`self.Event Add Countdown Time`)
    (else
      (bind _releasedactor (`self.ReleaseFromParent` 1500.0))
      (bind _asbp_kitchen_timer (cast `/Game/Items/Utility/BP_KitchenTimer` _releasedactor))
      (set `/Game/Items/Utility/BP_KitchenTimer.Timer` (`self.Timer`) _asbp_kitchen_timer)
      (if (`self.Countdown?`)
        (`self.Event Start Countdown` _asbp_kitchen_timer)))))

(event `self.Alt`
  (params (`Start?` :type Boolean))
  (if `Start?`
    (`self.Event Add Countdown Time`)))

(event `Event Add Countdown Time`
  (set `self.Timer` (+ (`self.Timer`) 5.0))
  (`self.SetDialRotation`)
  (`self.Event Start Countdown`))

(event `Event Start Countdown`
  (set `self.Countdown?` true)
  (bind _returnvalue (`KismetSystemLibrary.K2_SetTimerDelegate` (delegate `Event Countdown Tick`) (`self.TickDuration`) true true))
  (set `self.TimerHandle` _returnvalue))

(event `self.ReceiveHit`
  (params (MyComp :type "PrimitiveComponent Object Reference") (Other :type "Actor Object Reference") (OtherComp :type "PrimitiveComponent Object Reference") (bSelfMoved :type Boolean) (HitLocation :type "Vector Structure") (HitNormal :type "Vector Structure") (NormalImpulse :type "Vector Structure") (Hit :type "HitResult Structure (by ref)"))
  (`parent.ReceiveHit` MyComp Other OtherComp bSelfMoved HitLocation HitNormal NormalImpulse Hit)
  (`GameplayStatics.ApplyDamage` Other 1.0 null null "/Game/ElementalDamage/Kinetic/DTBP_Kinetic.DTBP_Kinetic_C"))

(event `Event Countdown Tick`
  (set `self.Timer` (- (`self.Timer`) (`self.TickDuration`)))
  (`self.SetDialRotation`)
  (if (<= (`self.Timer`) 0.0)
    (`self.Event Alarm`)
    (else
      (`GameplayStatics.PlaySoundAtLocation` (`self.TickSound`) (`self.K2_GetActorLocation`) (struct) 1.0 1.0 0.0 "/Game/Audio/AttenuationPresets/ATT_Default.ATT_Default" null null null))))

(event `Event Alarm`
  (bind _returnvalue (`self.K2_GetActorLocation`))
  (`GameplayStatics.PlaySoundAtLocation` (`self.AlarmSound`) _returnvalue (struct) 1.0 1.0 0.0 "/Game/Audio/AttenuationPresets/ATT_Default.ATT_Default" null null null)
  (`AISense_Hearing.ReportNoiseEvent` _returnvalue 1.0 (select `bool` (`self.ParentIsCharacter?`) :`false` self :`true` (`self.ParentActor`) :!type "Actor Object Reference") 1000.0)
  (`KismetSystemLibrary.K2_ClearAndInvalidateTimerHandle` (`self.TimerHandle`))
  (set `self.Countdown?` false))

(fn `SetDialRotation`
  (`SceneComponent.K2_SetRelativeRotation` (`self.Dial`) (`KismetMathLibrary.MakeRotator` 0.0 (* (`self.Timer`) 10.0)) false false))

(fn `UserConstructionScript`
  (`parent.UserConstructionScript`))