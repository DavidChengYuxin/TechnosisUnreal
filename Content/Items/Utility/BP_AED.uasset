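; BP_AED is an equippable, single-use defibrillator item that plays a startup sound and disables its mesh collision when spawned with a parent actor.
; Trigger fires Shock once, which plays the use sound, applies damage, then despawns the equipped item after a short delay.
; Damage is two full-strength radial hits that ignore the parent actor: wide electricity damage, plus a smaller-radius heal delivered through a heal damage type.
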(event `self.ReceiveBeginPlay`
  (`parent.ReceiveBeginPlay`)
  (`/Engine/EditorBlueprintResources/StandardMacros.IsValid` (`self.ParentActor`)
    (:`Is Valid`
      (`GameplayStatics.PlaySound2D` (`self.AEDStartUp`) 1.0 1.0 0.0 null (`self.ParentActor`) false)
      (bind _meshcompoments (`/Game/Universal/BPFL_Universal.Get All Mesh Components` self))
      (for _array_element _meshcompoments
        (`PrimitiveComponent.SetCollisionEnabled` _array_element "NoCollision")))))

(event `/Game/Items/BPI_Item.Trigger`
  (params (`Start?` :type Boolean))
  (if `Start?`
    (`/Engine/EditorBlueprintResources/StandardMacros.DoOnce` false
      (:`Completed`
        (`self.Event Shock`)))))

(event `Event Shock`
  (bind _parentactor (`self.ParentActor`))
  (bind _parentactor_2 (`self.ParentActor`))
  (bind _returnvalue (`SceneComponent.K2_GetComponentLocation` (`self.ShockLocation`)))
  (`GameplayStatics.PlaySound2D` (`self.AEDUse`) 1.0 1.0 0.0 null (`self.ParentActor`) false)
  (`GameplayStatics.ApplyRadialDamage` 200.0 _returnvalue 300.0 "/Game/ElementalDamage/Electricity/DTBP_Electricity.DTBP_Electricity_C" (`|MakeArray` _parentactor_2) _parentactor_2 (`self.GetInstigatorController` _parentactor_2) true "ECC_Camera")
  (`GameplayStatics.ApplyRadialDamage` 35.0 _returnvalue 100.0 "/Game/ElementalDamage/Heal/DTBP_Heal.DTBP_Heal_C" (`|MakeArray` _parentactor) _parentactor (`self.GetInstigatorController` _parentactor) true "ECC_Camera")
  (`KismetSystemLibrary.Delay` 0.5)
  (`self.DespawnWhileEquipped`))

(fn `UserConstructionScript`
  (`parent.UserConstructionScript`))