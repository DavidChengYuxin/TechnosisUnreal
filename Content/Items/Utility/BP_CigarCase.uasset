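; BP_CigarCase is an interactable utility item actor for a cigar case.
; Its construction script runs the parent setup, then sets the interaction type on its BPCInteractable component.
; The Interact event only branches on InteractStart with nothing connected, so interacting has no effect in this Blueprint.
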(event `/Game/Universal/Interact/BPI_Interact.Interact`
  (params (`InteractStart?` :type Boolean) (Causer :type "Actor Object Reference") (Instigator :type "Controller Object Reference"))
  (if `InteractStart?`
    _))

(fn `UserConstructionScript`
  (`parent.UserConstructionScript`)
  (set `/Game/Universal/Interact/BPC_Interactable.InteractionType` "NewEnumerator4" (`self.BPC_Interactable`)))