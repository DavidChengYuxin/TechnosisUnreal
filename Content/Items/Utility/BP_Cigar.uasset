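; BP_Cigar is a usable utility item that plays smoking montages on its holder and deals fire damage to them per puff.
; Trigger spends puffs to set the lit state, consuming inventory on the first puff and resetting once puffs run out.
; Alt releases it; on hit, a lit cigar burns the target and self-destructs.
; Elemental damage alters burn, puffs or lit state; second-hand smoke code is unconnected.
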(event `self.ReceiveBeginPlay`
  (`|PlayMontage` (`self.ParentSkeletalMesh`) (`self.NewCigaretteAnim`)))

(event `/Game/Items/BPI_Item.Trigger`
  (params (`Start?` :type Boolean))
  (bind _parentactor (`self.ParentActor`))
  (bind _returnvalue (> (`self.Puffs`) 0))
  (if `Start?`
    (if _returnvalue
      (`/Engine/EditorBlueprintResources/StandardMacros.DecrementInt` (`self.Puffs`)
        (:`  `
          (set `self.CigaretteLit?` _returnvalue)
          (`|ExecutionSequence`
            (:`then_0`
              (`/Engine/EditorBlueprintResources/StandardMacros.DoOnce` false :!label _label
                (:`Completed`
                  (`self.Consume from Inventory`))))
            (:`then_1`
              (`|PlayMontage` (`self.ParentSkeletalMesh`) (`self.SmokeAnim`)))
            (:`then_2`
              (`GameplayStatics.ApplyDamage` _parentactor (`self.SmokeFireDuration`) (`self.GetInstigatorController` _parentactor) _parentactor "/Game/ElementalDamage/Fire/DTBP_Fire.DTBP_Fire_C")))))
      (else
        (set `self.CigaretteLit?` false)
        (set `self.Puffs` (`self.MaxPuffs`))
        (`|PlayMontage` (`self.ParentSkeletalMesh`) (`self.NewCigaretteAnim`)
          (:`then`
            (goto _label :!via `Reset`)))))))

(event `self.ReceiveAnyDamage`
  (params (Damage :type "Float (single-precision)") (DamageType :type "DamageType Object Reference") (InstigatedBy :type "Controller Object Reference") (DamageCauser :type "Actor Object Reference"))
  (`/Game/Universal/BPML_Universal.SwitchOnElementalDamage` DamageType
    (:`Fire`
      (`/Game/ElementalDamage/Fire/BPC_Flammable.Event Add Burn Duration` (`self.BPC_Flammable`) Damage)
      (set `self.Puffs` 0))
    (:`Ice`
      (set `self.CigaretteLit?` false :!label _label_2))
    (:`Water`
      (set `self.Puffs` 0)
      (goto _label_2))))

(event `/Game/Items/BPI_Item.Alt`
  (params (`Start?` :type Boolean))
  (`self.ReleaseFromParent` 50.0))

(event `self.ReceiveHit`
  (params (MyComp :type "PrimitiveComponent Object Reference") (Other :type "Actor Object Reference") (OtherComp :type "PrimitiveComponent Object Reference") (bSelfMoved :type Boolean) (HitLocation :type "Vector Structure") (HitNormal :type "Vector Structure") (NormalImpulse :type "Vector Structure") (Hit :type "HitResult Structure (by ref)"))
  (bind _parentactor (`self.ParentActor`))
  (if (`self.CigaretteLit?`)
    (`GameplayStatics.ApplyDamage` Other 5.0 (`self.GetInstigatorController` _parentactor) _parentactor "/Game/ElementalDamage/Fire/DTBP_Fire.DTBP_Fire_C")
    (`NiagaraFunctionLibrary.SpawnSystemAttached` "/Game/Effects/StarterContent/NS_Fire.NS_Fire" null "None" HitLocation (struct) "KeepRelativeOffset" true)
    (`self.K2_DestroyActor`)
    (elif (<= (`self.Puffs`) 0)
      (`self.K2_DestroyActor`))))

(event `Event Smoke Cigarette`)

(fn `UserConstructionScript`
  (`parent.UserConstructionScript`))