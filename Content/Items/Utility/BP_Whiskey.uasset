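; BP_Whiskey is a drinkable, throwable whiskey bottle item with limited uses.
; Drinking plays a sip sound and tilt timeline, then heals the holder through ApplyDamage with a heal damage type.
; Alt releases it; hard impacts shatter it with glass, sound and AI noise, leaving an oil puddle.
; Damage reactions depend on element: fire or armor-piercing triggers radial damage, while blunt types shatter it or destroy it if empty.
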(event `Event Heal`
  (bind _parentactor (`self.ParentActor`))
  (`|ExecutionSequence`
    (:`then_0`
      (`GameplayStatics.PlaySound2D` "/Game/SoundEffects/FreeSound/sheyvan/471078__sheyvan__sipping-drink.471078__sheyvan__sipping-drink" 1.0 1.0 0.0 null null))
    (:`then_1`
      (bind (_direction _rotation) (`Timeline|Timeline` :!via `PlayFromStart`)
        (:`Update`
          (`SceneComponent.K2_SetRelativeRotation` (`self.Mesh`) (`KismetMathLibrary.MakeRotator` 0.0 (* _rotation -45.0)) false false))
        (:`Finished`
          (`GameplayStatics.ApplyDamage` _parentactor 5.0 (`self.GetInstigatorController` _parentactor) _parentactor "/Game/ElementalDamage/Heal/DTBP_Heal.DTBP_Heal_C"))))))

(event `self.ReceiveAnyDamage`
  (params (Damage :type "Float (single-precision)") (DamageType :type "DamageType Object Reference") (InstigatedBy :type "Controller Object Reference") (DamageCauser :type "Actor Object Reference"))
  (bind _parentactor (`self.ParentActor`))
  (switch `/Game/ElementalDamage/Enum_Element` (`/Game/Universal/BPFL_Universal.Get Element` DamageType)
    (:`NewEnumerator0`
      (if (`self.EmptyBottle?`) :!label _label
        (`self.K2_DestroyActor` :!label _label_2)
        (`self.Consume from Inventory`)
        (else
          (`self.Event Shatter Bottle`))))
    (:`NewEnumerator1`
      (`GameplayStatics.ApplyRadialDamageWithFalloff` :`Origin` (`self.K2_GetActorLocation`) :`DamageTypeClass` "/Game/ElementalDamage/ArmorPiercing/DTBP_ArmorPiercing.DTBP_ArmorPiercing_C" :`DamageCauser` _parentactor :`InstigatedByController` (`self.GetInstigatorController` _parentactor) :!label _label_3)
      (goto _label_2))
    (:`NewEnumerator8`
      (goto _label_3))
    (:`NewEnumerator7`
      (goto _label))
    (:`NewEnumerator4`
      (goto _label))))

(event `self.Trigger`
  (params (`Start?` :type Boolean))
  (bind _returnvalue (> (`self.Uses`) 0))
  (if `Start?`
    (if _returnvalue
      (`/Engine/EditorBlueprintResources/StandardMacros.DecrementInt` (`self.Uses`)
        (:`  `
          (set `self.EmptyBottle?` (not _returnvalue))
          (`self.Event Heal`)
          (`/Engine/EditorBlueprintResources/StandardMacros.DoOnce` false :!label _label_4
            (:`Completed`
              (`self.Consume from Inventory`)))))
      (else
        (set `self.Uses` (`self.MaximumUses`))
        (goto _label_4 :!via `Reset`)))))

(event `self.Alt`
  (params (`Start?` :type Boolean))
  (`self.ReleaseFromParent` 1500.0))

(event `self.ReceiveHit`
  (params (MyComp :type "PrimitiveComponent Object Reference") (Other :type "Actor Object Reference") (OtherComp :type "PrimitiveComponent Object Reference") (bSelfMoved :type Boolean) (HitLocation :type "Vector Structure") (HitNormal :type "Vector Structure") (NormalImpulse :type "Vector Structure") (Hit :type "HitResult Structure (by ref)"))
  (`parent.ReceiveHit` MyComp Other OtherComp bSelfMoved HitLocation HitNormal NormalImpulse Hit)
  (if (>= (`KismetMathLibrary.VSize` NormalImpulse) (`self.MinHitImpulse`))
    (`self.Event Shatter Bottle`)
    (if (== (`KismetArrayLibrary.Array_Length` (`self.GetOverlappingActors` "/Game/ElementalDamage/Fire/BP_OilPuddle.BP_OilPuddle_C")) 0)
      (`|SpawnActorFromClass` "/Game/ElementalDamage/Fire/BP_OilPuddle.BP_OilPuddle_C" (`KismetMathLibrary.MakeTransform` HitLocation) "Undefined" "MultiplyWithRoot" null null))))

(event `Event Shatter Bottle`
  (bind (_returnvalue_location _returnvalue_rotation) (`KismetMathLibrary.BreakTransform` (`self.GetTransform`)))
  (`NiagaraFunctionLibrary.SpawnSystemAtLocation` (`self.GlassShard`) _returnvalue_location _returnvalue_rotation)
  (`GameplayStatics.SpawnSoundAtLocation` "/Game/SoundEffects/FreeSound/spookymodern/202093__spookymodem__bottle-shattering.202093__spookymodem__bottle-shattering" _returnvalue_location (struct) 1.0 1.0 0.0 null null)
  (`AISense_Hearing.ReportNoiseEvent` _returnvalue_location 1.0 null 500.0)
  (`self.K2_DestroyActor`))

(fn `Spawn Alcohol Puddle`
  (params (Instigator :type "Pawn Object Reference"))
  (locals (PuddleScale :type "Float (double-precision)" :default 0.5))
  (bind _returnvalue (`self.K2_GetActorLocation`))
  (bind _puddlescale (`local.PuddleScale`))
  (bind (_outhit _returnvalue_2) (`KismetSystemLibrary.LineTraceSingle` _returnvalue (+ _returnvalue (* (`KismetMathLibrary.Vector_Down`) 50.0)) "TraceTypeQuery1"))
  (if _returnvalue_2
    (bind (_bblockinghit _binitialoverlap _time _distance _location _impactpoint _normal _impactnormal) (`GameplayStatics.BreakHitResult` _outhit))
    (`|SpawnActorFromClass` "/Game/ElementalDamage/Fire/BP_OilPuddle.BP_OilPuddle_C" (`KismetMathLibrary.MakeTransform` _impactpoint (`KismetMathLibrary.MakeRotFromZ` _impactnormal) (`KismetMathLibrary.MakeVector` _puddlescale _puddlescale 1.0)) "Undefined" "MultiplyWithRoot" null (`local.Instigator`))
    (`self.Event Shatter Bottle`)
    (else
      (`self.Event Shatter Bottle`))))

(fn `UserConstructionScript`
  (`parent.UserConstructionScript`))