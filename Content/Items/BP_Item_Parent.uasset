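; Base item actor that works either as a physics pickup in the world or as an item attached to a parent such as the player character.
; Construction either caches the parent player's camera, mesh and motion-matching AnimBP, or enables physics and interaction.
; Interacting adds it to the causer's inventory, pulls it toward their head by mass-scaled impulse, plays a sound and despawns if required.
; Release decrements inventory, detaches and restores physics, with optional forward throw impulse.
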(event `self.ReceiveBeginPlay`)

(event `/Game/Universal/Interact/BPI_Interact.Interact`
  (params (`InteractStart?` :type Boolean) (Causer :type "Actor Object Reference") (Instigator :type "Controller Object Reference"))
  (bind _shoulddespawn_ (`self.OnTaken` Causer))
  (`GameplayStatics.PlaySound2D` (`self.GetTakenSound`) 1.0 1.0 0.0 null null)
  (if _shoulddespawn_
    (`KismetSystemLibrary.Delay` 0.2)
    (`self.K2_DestroyActor`)))

(fn `Consume from Inventory`
  (locals (ParentInventory :type "/Game/Items/BPC_Inventory Object Reference"))
  (bind _returnvalue (`self.GetComponentByClass` (`self.ParentActor`) "/Game/Items/BPC_Inventory.BPC_Inventory_C"))
  (`/Engine/EditorBlueprintResources/StandardMacros.IsValid` _returnvalue
    (:`Is Valid`
      (bind _output_get (set `local.ParentInventory` _returnvalue))
      (`/Game/Items/BPC_Inventory.DecrementItem` _output_get (`.RowName` (break `DataTableRowHandle` (`self.ItemName`))) (0.0 0.0)))))

(fn `GetAmmo`
  (returns (Ammo :type Integer))
  (return 0))

(fn `GetTakenSound`
  (returns (OnTakenSound :type "SoundBase Object Reference"))
  (bind _ontakensounds (`self.OnTakenSounds`))
  (return (`|GetArrayItem` _ontakensounds (`KismetMathLibrary.RandomInteger` (- (`KismetArrayLibrary.Array_Length` _ontakensounds) 1)))))

(fn `On Take Add Impulse`
  (params (Causer :type "Actor Object Reference") (`DespawnItem?` :type Boolean))
  (locals (TakeVelocity :type "Float (double-precision)" :default 300.0) (DespawnVelocity :type "Float (double-precision)" :default 800.0))
  (bind _causer (`local.Causer`))
  (bind (_ascharacter _bsuccess) (cast `Character` _causer :!pure true))
  ;[1 1 1] Add impulse while grabbing
  (bind _meshcompoments (`/Game/Universal/BPFL_Universal.Get All Mesh Components` self))
  (for _array_element _meshcompoments
    (`PrimitiveComponent.AddImpulseAtLocation` _array_element (* (`KismetMathLibrary.GetDirectionUnitVector` (`self.K2_GetActorLocation`) (select `bool` _bsuccess :`false` (`self.K2_GetActorLocation` _causer) :`true` (`SceneComponent.GetSocketLocation` (`self.GetComponentByClass` _ascharacter "/Script/Engine.SkeletalMeshComponent") "head"))) (`PrimitiveComponent.GetMass` _array_element) (select `bool` (`local.DespawnItem?`) :`false` (`local.TakeVelocity`) :`true` (`local.DespawnVelocity`))) (`self.K2_GetActorLocation`) "None")
    (if (`local.DespawnItem?`)
      (`PrimitiveComponent.SetEnableGravity` _array_element false))))

(fn `OnTaken`
  (params (Causer :type "Actor Object Reference") (ItemQuantity :type Integer :default 1) (AmmoType :type "/Game/Items/Weapons/Firearms/Enum_AmmoType Enum" :default "NewEnumerator0"))
  (returns (`ShouldDespawn?` :type Boolean) (RemainderQuantity :type Integer))
  (locals (`DespawnItem?` :type Boolean :default false))
  (bind _returnvalue (`self.GetComponentByClass` (`local.Causer`) "/Game/Items/BPC_Inventory.BPC_Inventory_C"))
  (if (and (`|EnumEquality` (`/Game/Universal/Interact/BPC_Interactable.InteractionType` (`self.BPC_Interactable`)) "NewEnumerator4") (`KismetSystemLibrary.IsValid` _returnvalue))
    (bind (_remainderquantity _despawnitem_) (`/Game/Items/BPC_Inventory.AddItem` _returnvalue (`self.GetItemName`) (`local.ItemQuantity`) (`local.AmmoType`)))
    (set `local.DespawnItem?` _despawnitem_)
    (`|ExecutionSequence`
      (:`then_0`
        (`self.On Take Add Impulse` (`local.Causer`) (`local.DespawnItem?`)))
      (:`then_1`
        (return (`local.DespawnItem?`) _remainderquantity)))))

(fn `ReleaseFromParent`
  (params (ImpulseMagnitude :type "Float (double-precision)"))
  (locals (ForwardVector :type "Vector Structure"))
  (bind _parentactor (`self.ParentActor`))
  (`self.Consume from Inventory`)
  ;[1 1 1] Only get forward vector if adding impulse while releasing from parent. No impulse if ImpulseMagnitude 0.
  (if (> ImpulseMagnitude 0.0)
    (if (`KismetMathLibrary.ClassIsChildOf` (`GameplayStatics.GetObjectClass` (`self.ParentActor`)) "/Game/Player/Blueprints/BP_PlayerCharacter.BP_PlayerCharacter_C")
      (bind _asbp_player_character (cast `/Game/Player/Blueprints/BP_PlayerCharacter` _parentactor)
        (:`then`
          (set `local.ForwardVector` (`SceneComponent.GetForwardVector` (`/Game/Player/Blueprints/BP_PlayerCharacter.1stPersonCamera` _asbp_player_character))))
        (:`CastFailed`
          (set `local.ForwardVector` (`self.GetActorForwardVector` _parentactor) :!label _label)))
      (else
        (goto _label))))
  (`self.K2_DetachFromActor` "KeepRelative")
  (set `self.ParentActor` null)
  (set `self.ParentIsCharacter?` false)
  (`self.SetAsPhysicsObject`)
  (set `/Game/Universal/Interact/BPC_Interactable.InteractionType` "NewEnumerator4" (`self.BPC_Interactable`))
  (if (> (`local.ImpulseMagnitude`) 0.0)
    (bind _meshcompoments (`/Game/Universal/BPFL_Universal.Get All Mesh Components` self))
    (for _array_element _meshcompoments
      (`PrimitiveComponent.AddImpulseAtLocation` _array_element (* (`local.ForwardVector`) (`local.ImpulseMagnitude`)) (`self.K2_GetActorLocation`) "None"))))

(fn `SetAsPhysicsObject`
  (bind _meshcompoments (`/Game/Universal/BPFL_Universal.Get All Mesh Components` self))
  (for _array_element _meshcompoments
    (`PrimitiveComponent.SetCollisionProfileName` _array_element "BlockAll" false)
    (`PrimitiveComponent.SetSimulatePhysics` _array_element true)
    (`PrimitiveComponent.SetMassOverrideInKg` _array_element "None" (`self.Mass`) true)))

(fn `SetUpParent`
  (bind _output_get (set `self.ParentActor` (`self.GetParentActor`)))
  (bind _asbp_player_character (cast `/Game/Player/Blueprints/BP_PlayerCharacter` _output_get))
  ;[1 1 1] Sets reference object, currently uses first person camera
  (set `self.OwnerReferenceComponent` (`/Game/Player/Blueprints/BP_PlayerCharacter.1stPersonCamera` _asbp_player_character))
  (bind _mesh (`Character.Mesh` _asbp_player_character))
  (set `self.ParentSkeletalMesh` _mesh)
  (bind _asabp_motion_matching (cast `/Game/Animations/ABP_MotionMatching` (`SkeletalMeshComponent.GetAnimInstance` _mesh)))
  (set `self.As ABP` _asabp_motion_matching)
  (set `self.ParentIsCharacter?` true))

(fn `UserConstructionScript`
  (`/Engine/EditorBlueprintResources/StandardMacros.IsValid` (`self.GetParentActor`)
    (:`Is Valid`
      (`self.SetUpParent`))
    (:`Is Not Valid`
      (`self.SetAsPhysicsObject`)
      (set `/Game/Universal/Interact/BPC_Interactable.InteractionType` "NewEnumerator4" (`self.BPC_Interactable`)))))