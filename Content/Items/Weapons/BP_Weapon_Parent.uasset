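; Base weapon actor for held, pickup-able guns, providing firing, ammo, reloading, recoil and spread.
; Trigger routes through single, burst or timer-driven full-auto modes into SingleAttack, which fires a hitscan trace with per-bone damage or spawns a projectile.
; Montage-driven reload draws from the owner's BPC_Inventory reserve, or fills the magazine without one.
; Shots report AI noise unless silenced, feed AnimBP recoil, and enable Tick only while hitscan spread recovers.
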(event `self.ReceiveTick`
  (params (DeltaSeconds :type "Float (single-precision)"))
  ;[1 1 1] Event Tick used to shrink spread. Turn off when spread == 0.
  (if (`|EnumEquality` (`self.AttackMethod`) "NewEnumerator0")
    (bind _output_get (set `self.HitScanSpread` (- (`self.HitScanSpread`) (* DeltaSeconds (`self.RPM`) 0.01666 (`self.SpreadRecoveryRate`)))))
    (if (<= _output_get 0.0)
      (`self.SetActorTickEnabled` false :!label _label)
      (set `self.HitScanSpread` 0.0))
    (else
      (goto _label))))

(event `/Game/Items/BPI_Item.Trigger`
  (params (`Start?` :type Boolean))
  (bind _output_get (set `self.Triggered?` `Start?`))
  (if _output_get
    (`self.HasAmmo?`
      (:`HasAmmo`
        ;[1 1 1] Start triggered
        (switch `/Game/Items/Weapons/Enum_WeaponMode` (`self.WeaponMode`)
          (:`NewEnumerator0`
            (`/Engine/EditorBlueprintResources/StandardMacros.DoOnce` false :!label _label_2
              (:`Completed`
                (`self.SingleAttack`))))
          (:`NewEnumerator1`
            (`/Engine/EditorBlueprintResources/StandardMacros.DoOnce` false :!label _label_3
              (:`Completed`
                (bind _returnvalue (`KismetSystemLibrary.K2_SetTimerDelegate` (delegate `Event Burst`) (`self.HitDelay`) true true))
                (set `self.BurstTimerHandle` _returnvalue)
                (`self.Event Burst`))))
          (:`NewEnumerator2`
            (bind _returnvalue_2 (`KismetSystemLibrary.K2_SetTimerDelegate` (delegate `Event Automatic`) (`self.HitDelay`) true true))
            (`self.Event Automatic`))))
      (:`NoAmmo`
        (`/Game/Items/BPI_Item.Reload`)))
    (else
      ;[1 1 1] Stop triggered
      (switch `/Game/Items/Weapons/Enum_WeaponMode` (`self.WeaponMode`)
        (:`NewEnumerator0`
          (goto _label_2 :!via `Reset`))
        (:`NewEnumerator1`
          (`KismetSystemLibrary.Delay` (`self.DelayBetweenBurst`))
          (goto _label_3 :!via `Reset`))
        (:`NewEnumerator2`
          (`KismetSystemLibrary.K2_ClearAndInvalidateTimerHandle` _returnvalue_2))))))

(event `/Game/Items/BPI_Item.Reload`
  (bind _returnvalue (`self.GetComponentByClass` (`self.ParentActor`) "/Game/Items/BPC_Inventory.BPC_Inventory_C"))
  (bind _returnvalue_2 (`self.GetComponentByClass` (`self.ParentActor`) "/Game/Items/BPC_Inventory.BPC_Inventory_C"))
  (bind (_value _returnvalue_3) (`BlueprintMapLibrary.Map_Find` (`/Game/Items/BPC_Inventory.AmmoReserve` _returnvalue) (`self.AmmoType`)))
  (bind (_value_2 _returnvalue_4) (`BlueprintMapLibrary.Map_Find` (`/Game/Items/BPC_Inventory.AmmoReserve` _returnvalue_2) (`self.AmmoType`)))
  ;[1 1 1] Reload
  (if (and (`self.ReloadReady?`) (or (not (`KismetSystemLibrary.IsValid` _returnvalue_2)) (not (`/Game/Items/BPC_Inventory.FiniteAmmo?` _returnvalue_2)) (!= _value_2 0) (not _returnvalue_4)))
    (set `self.ReloadReady?` false)
    (`|PlayMontage` (`self.GetComponentByClass` (`self.ParentActor`) "/Script/Engine.SkeletalMeshComponent") (`self.ReloadAnim`)
      (:`then`
        (goto _label_4 :!via `Reset`))
      (:`OnCompleted`
        (`/Engine/EditorBlueprintResources/StandardMacros.DoOnce` false :!label _label_4
          (:`Completed`
            (set `self.ReloadReady?` true)
            (if (`self.FiniteAmmo?`)
              (if (and (`KismetSystemLibrary.IsValid` _returnvalue) (`/Game/Items/BPC_Inventory.FiniteAmmo?` _returnvalue) _returnvalue_3)
                (`self.Loads Ammo Iff Finite Ammo` _value)
                (else
                  ;;[1 1 1] If parent has no inventory, treat as having infinite ammo
                  (set `self.Ammo` (`self.MaxAmmo`))))))))
      (:`OnInterrupted`
        (set `self.ReloadReady?` true))
      (:`OnNotifyBegin`
        (goto _label_4)))))

(event `Event Burst`
  (bind _burstcounter (`self.BurstCounter`))
  (`self.SingleAttack`)
  (`/Engine/EditorBlueprintResources/StandardMacros.IncrementInt` _burstcounter
    (:`  `
      (if (>= _burstcounter (`self.HitsPerBurst`))
        (`KismetSystemLibrary.K2_ClearAndInvalidateTimerHandle` (`self.BurstTimerHandle`))
        (set `self.BurstCounter` 0)))))

(event `Event Automatic`
  (`self.SingleAttack`))

(event `/Game/Universal/Interact/BPI_Interact.Interact`
  (params (`InteractStart?` :type Boolean) (Causer :type "Actor Object Reference") (Instigator :type "Controller Object Reference"))
  ;[1 1 1] On Taken
  (bind (_shoulddespawn_ _remainderquantity) (`self.OnTaken` Causer (`self.Ammo`) (`self.AmmoType`)))
  (if _shoulddespawn_
    (`GameplayStatics.PlaySound2D` (`self.GetTakenSound`) 1.0 1.0 0.0 null null)
    (`KismetSystemLibrary.Delay` 0.25)
    (`self.K2_DestroyActor`)
    (else
      (set `self.Ammo` _remainderquantity))))

(event `Event Add Spread`
  (`/Engine/EditorBlueprintResources/StandardMacros.IncrementFloat` (`self.HitScanSpread`)
    (:`  `
      (`self.SetActorTickEnabled` true))))

(event `/Game/Items/BPI_Item.SetAmmo`
  (params (Ammo :type Integer))
  ;[1 1 1] Set & get ammo (usually on equip)
  (set `self.Ammo` (`KismetMathLibrary.Clamp` Ammo 0 (`self.MaxAmmo`))))

(event `/Game/Items/BPI_Item.NewParent`
  (params (OwnerReferenceComponent :type "Actor Object Reference"))
  (`self.SetUpParent`)
  (`self.Set Up Anim`))

(event `self.Box.OnComponentBeginOverlap`
  (params (OverlappedComponent :type "PrimitiveComponent Object Reference") (OtherActor :type "Actor Object Reference") (OtherComp :type "PrimitiveComponent Object Reference") (OtherBodyIndex :type Integer) (bFromSweep :type Boolean) (SweepResult :type "HitResult Structure (by ref)"))
  (switch `/Game/Items/Weapons/Enum_AttackMethod` (`self.AttackMethod`)))

(fn `AddRecoil`
  (bind _as_abp (`self.As ABP`))
  (if (and (`self.ParentIsCharacter?`) (`self.HasRecoil?`))
    (set `/Game/Animations/ABP_MotionMatching.RecoilAlpha` (`KismetMathLibrary.FClamp` (+ (`/Game/Animations/ABP_MotionMatching.RecoilAlpha` _as_abp) (`self.RecoilPercentPerTrigger`))) _as_abp)))

(fn `GetAmmo`
  (returns (Ammo :type Integer))
  (return (`self.Ammo`)))

(fn `Impact Sound And Decal`
  (params (ImpactDecal :type "MaterialInterface Object Reference") (ImpactSound :type "SoundBase Object Reference") (ImpactLocation :type "Vector Structure") (ImpactNormal :type "Vector Structure"))
  (locals (DecalSize :type "Float (double-precision)" :default 1.0) (DecalDuration :type "Float (double-precision)" :default 30.0) (SoundLoudness :type "Float (double-precision)" :default 0.2) (SoundRange :type "Float (double-precision)" :default 500.0))
  (`GameplayStatics.SpawnDecalAtLocation` ImpactDecal (`KismetMathLibrary.Conv_DoubleToVector` (`local.DecalSize`)) ImpactLocation (`KismetMathLibrary.Conv_VectorToRotator` ImpactNormal) (`local.DecalDuration`))
  (`self.Spawn Particle & Sound` null ImpactSound ImpactLocation (struct) (`local.SoundLoudness`) (`local.SoundRange`)))

(fn `Loads Ammo Iff Finite Ammo`
  (params (OwnerAmmoCount :type Integer))
  (locals (DeltaAmmo :type Integer))
  (bind _deltaammo (`self.MagazineVacancy`))
  (bind _output_get (set `local.DeltaAmmo` (select `bool` (>= (`local.OwnerAmmoCount`) _deltaammo) :`false` OwnerAmmoCount :`true` _deltaammo)))
  (set `self.Ammo` (+ _output_get (`self.Ammo`)))
  ;[1 1 1] Updates player ammo pool
  (`BlueprintMapLibrary.Map_Add` (`/Game/Items/BPC_Inventory.AmmoReserve` (`self.GetComponentByClass` (`self.ParentActor`) "/Game/Items/BPC_Inventory.BPC_Inventory_C")) (`self.AmmoType`) (- (`local.OwnerAmmoCount`) (`local.DeltaAmmo`))))

(fn `Set Up Anim`
  (bind _parentactor (`self.ParentActor`))
  (`/Engine/EditorBlueprintResources/StandardMacros.IsValid` _parentactor
    (:`Is Valid`
      (message `/Game/Items/BPI_Item.SetOffHandIK` _parentactor (`self.OffHandIKTarget`) (`self.TwoHanded?`))
      (set `/Game/Animations/ABP_MotionMatching.MaxRecoil` (`self.MaxRecoilRotation`) (`self.As ABP`)))))

(fn `SingleAttack`
  (locals (Projectile :type "Actor Class Reference"))
  (bind _returnvalue (`self.GetParentActor`))
  (bind (_returnvalue_location _returnvalue_rotation) (`KismetMathLibrary.BreakTransform` (`SceneComponent.K2_GetComponentToWorld` (`self.MuzzleSocket`))))
  (bind (_start _end) (`self.CharacterHitScanVectors` (`self.HitScanSpread`)))
  (`self.HasAmmo?`
    (:`HasAmmo`
      (`self.Spawn Particle & Sound` (`self.AttackParticle`) (`self.AttackSound`) _returnvalue_location _returnvalue_rotation (`self.AttackLoudness`) (`self.AttackSoundRange`))
      (if (`self.FiniteAmmo?`)
        (`/Engine/EditorBlueprintResources/StandardMacros.DecrementInt` (`self.Ammo`)
          (:`  `
            _)))
      (`|ExecutionSequence`
        (:`then_0`
          (switch `/Game/Items/Weapons/Enum_AttackMethod` (`self.AttackMethod`)
            (:`NewEnumerator0`
              (if true
                (bind (_outhit _returnvalue_2) (`KismetSystemLibrary.LineTraceSingle` _start _end "TraceTypeQuery2" false (`|MakeArray` (`self.ParentActor`))))
                (`self.Event Add Spread`)
                (if _returnvalue_2
                  (bind (_bblockinghit _binitialoverlap _time _distance _location _impactpoint _normal _impactnormal _physmat _hitactor _hitcomponent _hitbonename _bonename _hititem _elementindex _faceindex _tracestart) (`GameplayStatics.BreakHitResult` _outhit))
                  (`/Engine/EditorBlueprintResources/StandardMacros.IsValid` _hitactor
                    (:`Is Valid`
                      (bind (_value _returnvalue_3) (`BlueprintMapLibrary.Map_Find` (`self.PerBoneDamageMultiplier`) _hitbonename))
                      (`GameplayStatics.ApplyPointDamage` _hitactor (* (`self.DamagePerHit`) (select `bool` _returnvalue_3 :`false` 1.0 :`true` _value)) _tracestart _outhit (`self.GetInstigatorController` _returnvalue) _returnvalue (`/Game/Universal/BDML_Universal.GetElementalDamageClass` (`self.WeaponElement`))))
                    (:`Is Not Valid`
                      (`self.Impact Sound And Decal` null null _impactpoint _impactnormal))))))
            (:`NewEnumerator1`
              (`|SpawnActorFromClass` (`local.Projectile`) (`SceneComponent.K2_GetComponentToWorld` (`self.MuzzleSocket`)) "Undefined" "MultiplyWithRoot" null null))))
        (:`then_1`
          (`self.AddRecoil`))))
    (:`NoAmmo`
      (`GameplayStatics.PlaySound2D` (`self.NoAmmoSound`) 1.0 1.0 0.0 null null))))

(fn `Spawn Particle & Sound`
  (params (Particle :type "NiagaraSystem Object Reference") (Sound :type "SoundBase Object Reference") (Location :type "Vector Structure") (Rotation :type "Rotator Structure") (Loudness :type "Float (single-precision)") (MaxRange :type "Float (single-precision)"))
  (`NiagaraFunctionLibrary.SpawnSystemAtLocation` Particle Location Rotation)
  (`GameplayStatics.SpawnSoundAtLocation` Sound Location (struct) 1.0 1.0 0.0 null null)
  (if (not (`self.Silenced?`))
    (`AISense_Hearing.ReportNoiseEvent` Location Loudness (`self.GetInstigatorController` (`self.GetParentActor`)) MaxRange)))

(fn `UserConstructionScript`
  (`parent.UserConstructionScript`)
  (`self.Set Up Anim`))