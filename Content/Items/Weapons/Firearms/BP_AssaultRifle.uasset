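; BP_AssaultRifle is a firearm weapon Blueprint that switches between burst and full-auto fire.
; Alt input toggles the mode through a FlipFlop on press instead of aiming down sights, selecting burst first.
; Each mode event sets the weapon mode and its fire rate, with burst firing faster than full-auto.
; The actual firing logic is not in this graph, which only configures those variables.
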(event `/Game/Items/BPI_Item.Alt`
  (params (`Start?` :type Boolean))
  ;[1 1 1] Alt mode changes firing mode (does not ADS)
  (if `Start?`
    (`/Engine/EditorBlueprintResources/StandardMacros.FlipFlop`
      (:`A`
        (`self.Event Set Burst`))
      (:`B`
        (`self.Event Set Full Auto`)))))

(event `Event Set Full Auto`
  ;[1 1 1] Alt mode changes firing mode (does not ADS)
  (set `self.RPM` 650.0)
  (set `self.WeaponMode` "NewEnumerator2"))

(event `Event Set Burst`
  ;[1 1 1] Alt mode changes firing mode (does not ADS)
  (set `self.RPM` 800.0)
  (set `self.WeaponMode` "NewEnumerator1"))

(fn `UserConstructionScript`
  (`parent.UserConstructionScript`))