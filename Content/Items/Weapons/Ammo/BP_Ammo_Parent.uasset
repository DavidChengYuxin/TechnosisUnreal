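; Parent Blueprint for ammo pickups that add ammo to the interacting actor's inventory.
; On interact start, it passes its ammo type and quantity to the causer's BPC_Inventory and plays a 2D taken sound.
; A positive AddAmmo result swaps to the half-used mesh without updating the stored quantity.
; Otherwise it calls OnTakeAddImpulse with despawn set and destroys the actor after a short delay.
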(event `/Game/Universal/Interact/BPI_Interact.Interact`
  (params (`InteractStart?` :type Boolean) (Causer :type "Actor Object Reference") (Instigator :type "Controller Object Reference"))
  (bind _returnvalue (`self.GetComponentByClass` Causer "/Game/Items/BPC_Inventory.BPC_Inventory_C"))
  ;[1 1 1] Sanity check
  (if (and `InteractStart?` (`KismetSystemLibrary.IsValid` _returnvalue))
    (bind _remainderammo (`/Game/Items/BPC_Inventory.AddAmmo` _returnvalue (`self.AmmoQuantity`) (`self.AmmoType`)))
    (`GameplayStatics.PlaySound2D` (`self.GetTakenSound`) 1.0 1.0 0.0 null null)
    (if (> _remainderammo 0)
      (`StaticMeshComponent.SetStaticMesh` (`self.StaticMesh`) (`self.HalfUsedMesh`))
      (else
        (`self.On Take Add Impulse` Causer true)
        (if true
          (`KismetSystemLibrary.Delay` 0.2)
          (`self.K2_DestroyActor`))))))

(fn `UserConstructionScript`
  (`parent.UserConstructionScript`))