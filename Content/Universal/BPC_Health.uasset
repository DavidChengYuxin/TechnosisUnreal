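; Actor component that tracks its owner's health, handling damage, healing, unconsciousness and death, including on destruction or kill-volume overlap.
; Bound damage events read the damage type's BPI_Element to apply armor, sibling-component elemental modifiers or knockback impulses, then mostly report a damage event.
; Timers regenerate low health and drain overheal.
; Fire only reports here, its old logic deprecated as moved to a component; player death is marked work-in-progress.
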(event `self.ReceiveBeginPlay`
  (bind _returnvalue (`self.GetOwner`))
  (add `Actor.OnTakeAnyDamage` _returnvalue (delegate `EventOwnerRecieveDamage`))
  (add `Actor.OnTakePointDamage` _returnvalue (delegate `EventOwnerRecievePointDamage`))
  (add `Actor.OnTakeRadialDamage` _returnvalue (delegate `OwnerRecieveRadialDamage`))
  (add `Actor.OnDestroyed` _returnvalue (delegate `Event Owner Destroyed`))
  (add `Actor.OnActorBeginOverlap` _returnvalue (delegate `Event Overlap`)))

(event `Event Owner Destroyed`
  (params (DestroyedActor :type "Actor Object Reference"))
  (`self.Event Death`))

(event `EventOwnerRecieveDamage`
  (params (DamagedActor :type "Actor Object Reference") (Damage :type "Float (single-precision)") (DamageType :type "DamageType Object Reference") (InstigatedBy :type "Controller Object Reference") (DamageCauser :type "Actor Object Reference"))
  (`self.ProcessElementalDamage` Damage DamageType InstigatedBy DamageCauser))

(event `EventOwnerRecievePointDamage`
  (params (DamagedActor :type "Actor Object Reference") (Damage :type "Float (single-precision)") (InstigatedBy :type "Controller Object Reference") (HitLocation :type "Vector Structure") (FHitComponent :type "PrimitiveComponent Object Reference") (BoneName :type Name) (ShotFromDirection :type "Vector Structure") (DamageType :type "DamageType Object Reference") (DamageCauser :type "Actor Object Reference"))
  (`self.ProcessPointDamage` Damage DamageType InstigatedBy DamageCauser HitLocation ShotFromDirection BoneName))

(event `OwnerRecieveRadialDamage`
  (params (DamagedActor :type "Actor Object Reference") (Damage :type "Float (single-precision)") (DamageType :type "DamageType Object Reference") (Origin :type "Vector Structure") (HitInfo :type "HitResult Structure (by ref)") (InstigatedBy :type "Controller Object Reference") (DamageCauser :type "Actor Object Reference"))
  (bind (_bblockinghit _binitialoverlap _time _distance _location _impactpoint _normal _impactnormal _physmat _hitactor _hitcomponent _hitbonename) (`GameplayStatics.BreakHitResult` HitInfo))
  (`self.ProcessPointDamage` Damage DamageType InstigatedBy DamageCauser _impactpoint Origin _hitbonename))

(event `Event Overlap`
  (params (OverlappedActor :type "Actor Object Reference") (OtherActor :type "Actor Object Reference"))
  (if (`KismetMathLibrary.ClassIsChildOf` (`GameplayStatics.GetObjectClass` OtherActor) "/Script/Engine.KillZVolume")
    (`self.Event Death`)))

(event `Event Recieve Processed Damage`
  (params (Damage :type "Float (double-precision)"))
  (bind _output_get (set `self.Health` (- (`self.Health`) Damage)))
  (if (<= _output_get 0.0)
    (`self.Event Death`)
    (elif (< _output_get 20.0)
      (`KismetSystemLibrary.K2_SetTimerDelegate` (delegate `Event Health Regen Delay`) (`self.HealthRegenDelay`) false true))))

(event `Event Health Overflow Delay`
  (bind _returnvalue (`KismetSystemLibrary.K2_SetTimerDelegate` (delegate `Event Health Overflow`) (`GameplayStatics.GetWorldDeltaSeconds`) true true)))

(event `Event Health Regen Delay`
  ;[0.101 0.101 0.101] When health <20, start regenerating to 20
  (bind _returnvalue (`KismetSystemLibrary.K2_SetTimerDelegate` (delegate `Event Health Regen`) (`GameplayStatics.GetWorldDeltaSeconds`) true true)))

(event `Event Health Regen`
  ;[0.101 0.101 0.101] When health <20, start regenerating to 20
  (bind _output_get (set `self.Health` (+ (`self.Health`) (* (`GameplayStatics.GetWorldDeltaSeconds`) 10.0))))
  (if (> _output_get 20.0)
    (`KismetSystemLibrary.K2_ClearAndInvalidateTimerHandle` (stale `Event Health Regen Delay` _returnvalue))))

(event `Event Health Overflow`
  (bind _output_get (set `self.Health` (- (`self.Health`) (* (`GameplayStatics.GetWorldDeltaSeconds`) (`self.HealthOverflowDepletionRate`)))))
  (if (<= _output_get (`self.MaxHealth`))
    (`KismetSystemLibrary.K2_ClearAndInvalidateTimerHandle` (stale `Event Health Overflow Delay` _returnvalue))
    (if (> (`self.Health`) (- (`self.MaxHealth`) 1.0))
      (set `self.Health` (`self.MaxHealth`)))))

(event `Event Death`
  (`self.SetConscious` false)
  (`self.UnconsciousDispatcher`)
  (`self.DeathDispatcher`)
  (set `self.Alive?` false)
  ;[1 1 1] IFF player died - WORK IN PROGRESS
  (`/Engine/EditorBlueprintResources/StandardMacros.DoOnce` false
    (:`Completed`
      (bind _asbp_player_character (cast `/Game/Player/Blueprints/BP_PlayerCharacter` (`self.GetOwner`)))
      (`/Game/Player/Blueprints/BP_PlayerCharacter.Event On Death` _asbp_player_character))))

(event `Event Unconscious`
  (`self.SetConscious` false)
  (`self.UnconsciousDispatcher`))

(fn `ProcessArmorDamage`
  (params (IncomingDamage :type "Float (double-precision)"))
  (returns (OutgoingDamage :type "Float (double-precision)"))
  (locals (MinimumDamage :type "Float (double-precision)") (RatingToReductionMultiplier :type "Float (double-precision)" :default 12.0))
  (return (`KismetMathLibrary.FClamp` (- IncomingDamage (* (`self.ArmorRating`) (`local.RatingToReductionMultiplier`))) (`local.MinimumDamage`) IncomingDamage)))

(fn `ProcessElementalDamage`
  (params (Damage :type "Float (double-precision)") (DamageType :type "DamageType Object Reference") (InstigatedBy :type "Controller Object Reference") (DamageCauser :type "Actor Object Reference"))
  (locals (DamageElement :type "/Game/ElementalDamage/Enum_Element Enum" :default "NewEnumerator0"))
  (bind _returnvalue (`self.GetOwner`))
  (bind _returnvalue_2 (`self.GetOwner`))
  (bind _damage (`local.Damage`))
  (bind _damagecauser (`local.DamageCauser`))
  (bind _returnvalue_3 (`KismetSystemLibrary.IsValid` _damagecauser))
  (bind _returnvalue_4 (`Actor.GetComponentByClass` (`self.GetOwner`) "/Game/ElementalDamage/Ice/BPC_Freezable.BPC_Freezable_C"))
  (bind _returnvalue_5 (`Actor.GetComponentByClass` (`self.GetOwner`) "/Game/ElementalDamage/Ice/BPC_Freezable.BPC_Freezable_C"))
  (bind _returnvalue_6 (`Actor.GetComponentByClass` (`self.GetOwner`) "/Game/ElementalDamage/Water/BPC_WaterDamageable.BPC_WaterDamageable_C"))
  (bind _returnvalue_7 (select `bool` (select `bool` (`KismetSystemLibrary.IsValid` _returnvalue_5) :`true` (`/Game/ElementalDamage/Ice/BPC_Freezable.Frozen?` _returnvalue_5)) :`false` _damage :`true` (* _damage 2.0)))
  (if (`KismetSystemLibrary.DoesImplementInterface` DamageType "/Game/ElementalDamage/BPI_Element.BPI_Element_C")
    (bind _element (message `/Game/ElementalDamage/BPI_Element.GetElement` DamageType))
    (bind _output_get (set `local.DamageElement` _element))
    (switch `/Game/ElementalDamage/Enum_Element` _output_get
      (:`NewEnumerator0`
        (bind _outgoingdamage (`self.ProcessArmorDamage` _returnvalue_7))
        (`self.Event Recieve Processed Damage` _outgoingdamage)
        ;[0.05127 0.05127 0.05127] Report damage (to be reordered)
        (`AISense_Damage.ReportDamageEvent` _returnvalue (select `bool` _returnvalue_3 :`false` (`self.GetOwner`) :`true` _damagecauser) (`local.Damage`) (select `bool` _returnvalue_3 :`false` (`Actor.K2_GetActorLocation` _returnvalue) :`true` (`Actor.K2_GetActorLocation` _damagecauser)) :!label _label))
      (:`NewEnumerator1`
        (goto _label))
      (:`NewEnumerator2`
        (`/Engine/EditorBlueprintResources/StandardMacros.IsValid` (`Actor.GetComponentByClass` _returnvalue_2 "/Game/ElementalDamage/Electricity/BPC_Electrocutable.BPC_Electrocutable_C")
          (:`Is Valid`
            (`self.Event Recieve Processed Damage` (* (`local.Damage`) (select `bool` (`KismetSystemLibrary.IsValid` (`Actor.GetComponentByClass` _returnvalue_2 "/Game/ElementalDamage/Electricity/BPC_Conductive.BPC_Conductive_C")) :`false` 1.0 :`true` 2.0)))
            (goto _label))))
      (:`NewEnumerator3`
        (`/Engine/EditorBlueprintResources/StandardMacros.IsValid` _returnvalue_4
          (:`Is Valid`
            (`self.Event Recieve Processed Damage` (* (`/Game/ElementalDamage/Ice/BPC_Freezable.FrostbiteMultiplier` _returnvalue_4) (`local.Damage`))))))
      (:`NewEnumerator6`
        (`/Engine/EditorBlueprintResources/StandardMacros.IsValid` _returnvalue_6
          (:`Is Valid`
            (`self.Event Recieve Processed Damage` (* (`local.Damage`) (`/Game/ElementalDamage/Water/BPC_WaterDamageable.WaterDamageMultiplier` _returnvalue_6))))
          (:`Is Not Valid`)))
      (:`NewEnumerator8`
        (`self.Event Recieve Processed Damage` _returnvalue_7)
        (goto _label))
      (:`NewEnumerator7`
        (`self.EventKnockback`)
        (goto _label))
      (:`NewEnumerator9`
        (bind _output_get_2 (set `self.Health` (`KismetMathLibrary.FClamp` (+ (`self.Health`) (`KismetMathLibrary.Abs` (`local.Damage`))) 0.0 (* (`self.MaxHealth`) 2.0))))
        (if (> _output_get_2 (`self.MaxHealth`))
          (`self.Event Health Overflow Delay`)))
      (:`NewEnumerator4`
        (`self.Event Unconscious`)))
    (else
      ;[1 1 1] Processes non-elemental damage
      (`self.Event Recieve Processed Damage` (`local.Damage`)))))

(fn `ProcessPointDamage`
  (params (Damage :type "Float (double-precision)") (DamageType :type "DamageType Object Reference") (InstigatedBy :type "Controller Object Reference") (DamageCauser :type "Actor Object Reference") (HitLocation :type "Vector Structure") (ShotFromDirection :type "Vector Structure") (BoneName :type Name))
  (if (`KismetSystemLibrary.DoesImplementInterface` DamageType "/Game/ElementalDamage/BPI_Element.BPI_Element_C")
    (bind _element (message `/Game/ElementalDamage/BPI_Element.GetElement` (`local.DamageType`)))
    (switch `/Game/ElementalDamage/Enum_Element` _element
      (:`NewEnumerator7`
        (bind _meshcompoments (`/Game/Universal/BPFL_Universal.Get All Mesh Components` (`self.GetOwner`)))
        (for _array_element _meshcompoments
          (if (`SceneComponent.IsSimulatingPhysics` _array_element "None")
            (`PrimitiveComponent.AddImpulseAtLocation` _array_element (* (`local.Damage`) (`KismetMathLibrary.Normal` (`local.ShotFromDirection`))) (`local.HitLocation`) (`local.BoneName`))))))))

(fn `SetConscious`
  (params (`Conscious?` :type Boolean))
  (locals (AllSenseClasses :type "Array of AISense Class Reference") (`As BPC Interactable` :type "/Game/Universal/Interact/BPC_Interactable Object Reference"))
  (bind _output_get (set `self.Conscious?` `Conscious?`))
  (bind _asbp_npc_parent (cast `/Game/AI/BP_NPC_Parent` (`self.GetOwner`)))
  (message `/Game/AI/BPI_AI.SetConscious` _asbp_npc_parent _output_get))