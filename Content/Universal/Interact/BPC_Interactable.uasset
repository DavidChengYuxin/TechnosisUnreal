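; Actor component that makes its owner interactable, with only a work-in-progress Take interaction type handled.
; On Interact, Take applies a velocity-change impulse to the owner's static and skeletal meshes, toward the causer's "head" socket.
; The owner is destroyed after a short delay, giving a simple pickup effect.
; An alternative path that disables mesh collision is left disconnected.
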(event `/Game/Universal/Interact/BPI_Interact.Interact`
  (params (`InteractStart?` :type Boolean) (Causer :type "Actor Object Reference") (Instigator :type "Controller Object Reference"))
  (bind _returnvalue (`self.GetOwner`))
  (bind _returnvalue_2 (* (`KismetMathLibrary.GetDirectionUnitVector` (`Actor.K2_GetActorLocation` (`self.GetOwner`)) (`SceneComponent.GetSocketLocation` (`Actor.RootComponent` Causer) "head")) 50.0))
  (switch `/Game/Universal/Interact/Enum_Interaction` (`self.InteractionType`)
    (:`NewEnumerator4`
      ;[1 1 1] Taken (WORK IN PROGRESS)
      (`PrimitiveComponent.AddImpulse` (`Actor.K2_GetComponentsByClass` _returnvalue "/Script/Engine.StaticMeshComponent") _returnvalue_2 "None" true)
      (`PrimitiveComponent.AddImpulse` (`Actor.K2_GetComponentsByClass` _returnvalue "/Script/Engine.SkeletalMeshComponent") _returnvalue_2 "None" true)
      (`KismetSystemLibrary.Delay` 0.25)
      (`Actor.K2_DestroyActor` (`self.GetOwner`)))))